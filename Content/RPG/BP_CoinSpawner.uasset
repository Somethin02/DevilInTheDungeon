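; BP_CoinSpawner is a temporary actor that spawns a burst of BP_Coin actors at its own transform.
; SpawnCoins re-calls itself after a short delay, spawning one coin per pass until CoinsToSpawn is reached, then destroys the spawner.
; Each coin's LaunchCoin receives the spawner location and a yaw stepped by an equal share of 360 degrees, fanning coins in a ring.
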(event Custom|Spawn%20Coins
  (if (> (Variables|Default|GetCoinsToSpawn) (Variables|Default|GetCoins%20Spawned))
    (bind _returnvalue (Game|SpawnActorfromClass "/Game/RPG/BP_Coin.BP_Coin_C" (Transformation|GetActorTransform) "Undefined" "MultiplyWithRoot" 0 0))
    (Development|PrintString "coin spawned")
    (bind _result (Math|Integer|IncrementInt (Variables|Default|GetCoins%20Spawned))
      (:%20%20
        (Variables|Default|SetCoins%20Spawned _result)
        (Default|LaunchCoin _returnvalue (Math|Transform|MakeTransform (Transformation|GetActorLocation) (Math|Rotator|MakeRotator 0.0 0.0 (Math|Conversions|ToFloat(Integer) (* (/ 360 (Variables|Default|GetCoinsToSpawn)) (Variables|Default|GetCoins%20Spawned)))) "1.000000,1.000000,1.000000"))
        (Utilities|FlowControl|Delay 0.05)
        (CallFunction|SpawnCoins)))
    (else
      (Actor|DestroyActor))))

(event EventBeginPlay)

(event Collision|EventActorBeginOverlap
  (params (OtherActor :type Actor%20Object%20Reference)))

(event EventTick
  (params (DeltaSeconds :type Float%20%28single-precision%29)))

(fn ConstructionScript)