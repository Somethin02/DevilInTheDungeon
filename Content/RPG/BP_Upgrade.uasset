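; BP_Upgrade is an RPG pickup that boosts the active battle party when the overworld player overlaps it, then destroys itself.
; For each party member, it reads the StatName attribute and applies an ability-system effect to hard-coded "HP" using that value plus five, printing debug values.
; Launch arcs the Cube toward a destination via a suggested projectile velocity impulse; the accompanying path prediction drives no logic.
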(event OnComponentBeginOverlap(r)
  (params (OverlappedComponent :type Primitive%20Component%20Object%20Reference) (OtherActor :type Actor%20Object%20Reference) (OtherComp :type Primitive%20Component%20Object%20Reference) (OtherBodyIndex :type Integer) (bFromSweep :type Boolean) (SweepResult :type Hit%20Result%20Structure%20%28by%20ref%29))
  (Utilities|Casting|CastToBP_OverworldPlayerCharacter OtherActor)
  (bind _asbp_battle_character_controller (Utilities|Casting|CastToBP_BattleCharacterController (Game|GetPlayerController 0)))
  (for _array_element (Variables|/Game/RPG/BP_BattleCharacterController.BP_BattleCharacterController_C|GetActiveParty _asbp_battle_character_controller)
    (bind _asbp_player_actor (Utilities|Casting|CastToBP_PlayerActor _array_element))
    (bind _currentvalue_withmods_ (Default|GetAttributeCurrent (Variables|/Game/RPG/BP_TurnBasedActor.BP_TurnBasedActor_C|GetAC_AbilitySystem _asbp_player_actor) (Utilities|String|StringToName (Utilities|String|EnumtoString (Variables|Default|GetStatName)))))
    (Development|PrintString (Utilities|String|ToString(Float) (+ _currentvalue_withmods_ 5.0)) true true "(R=0.251335,G=1.000000,B=0.220595,A=1.000000)")
    (Default|ApplyEffecttoSelf (Variables|/Game/RPG/BP_TurnBasedActor.BP_TurnBasedActor_C|GetAC_AbilitySystem _asbp_player_actor) "NewEnumerator0" "HP" "NewEnumerator4" "NewEnumerator3" (+ _currentvalue_withmods_ 5.0))
    (bind _currentvalue_withmods__2 (Default|GetAttributeCurrent (Variables|/Game/RPG/BP_TurnBasedActor.BP_TurnBasedActor_C|GetAC_AbilitySystem _asbp_player_actor) (Utilities|String|StringToName (Utilities|String|EnumtoString (Variables|Default|GetStatName)))))
    (Development|PrintString (Utilities|String|ToString(Float) _currentvalue_withmods__2) true true "(R=1.000000,G=0.896004,B=0.019579,A=1.000000)"))
  (Actor|DestroyActor))

(event Custom|Launch
  (params (Destination :type Transform))
  (bind (_location _rotation) (Math|Transform|BreakTransform Destination))
  (bind _cube (Variables|Default|GetCube))
  (bind _returnvalue (Transformation|GetWorldLocation _cube))
  (bind _outlaunchvelocity (Game|SuggestProjectileVelocityCustomArc _returnvalue (+ _location (* (Math|Vector|GetForwardVector _rotation) 1e+01)) 0.0 0.5))
  (Variables|Default|SetOut%20Launch%20Velocity _outlaunchvelocity)
  (bind _returnvalue_2 (Class|GameplayStatics|BlueprintPredictProjectilePathAdvanced (Utilities|Struct|MakePredictProjectilePathParams _returnvalue _outlaunchvelocity false 0.0 5.0 true "ECC_WorldStatic" "ObjectTypeQuery1")))
  (if _returnvalue_2
    _
    (else
      _))
  (Class|PrimitiveComponent|AddVelocityChangeImpulseatLocation (Variables|Default|GetCube) (Variables|Default|GetOut%20Launch%20Velocity) (Transformation|GetWorldLocation (Variables|Default|GetCube)) "None"))

(event EventBeginPlay)

(event Collision|EventActorBeginOverlap
  (params (OtherActor :type Actor%20Object%20Reference)))

(event EventTick
  (params (DeltaSeconds :type Float%20%28single-precision%29)))

(fn ConstructionScript)