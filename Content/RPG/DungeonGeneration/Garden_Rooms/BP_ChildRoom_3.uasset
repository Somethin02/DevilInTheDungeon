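; BP_ChildRoom_3 is a garden room for RPG dungeon generation that controls its doors based on the player's presence.
; On BeginPlay it collects the children of SocketParent into a Sockets array.
; When the overworld player enters the PlayerCheck volume while the room is Locked, it shuts every BP_Door overlapping that volume.
; When the player leaves the volume, it reopens those overlapping doors regardless of the lock.
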(event OnComponentBeginOverlap(PlayerCheck)
  (params (OverlappedComponent :type Primitive%20Component%20Object%20Reference) (OtherActor :type Actor%20Object%20Reference) (OtherComp :type Primitive%20Component%20Object%20Reference) (OtherBodyIndex :type Integer) (bFromSweep :type Boolean) (SweepResult :type Hit%20Result%20Structure%20%28by%20ref%29))
  (Utilities|Casting|CastToBP_OverworldPlayerCharacter OtherActor)
  (if (Variables|Default|GetLocked)
    (CallFunction|ShutDoors)))

(event OnComponentEndOverlap(PlayerCheck)
  (params (OverlappedComponent :type Primitive%20Component%20Object%20Reference) (OtherActor :type Actor%20Object%20Reference) (OtherComp :type Primitive%20Component%20Object%20Reference) (OtherBodyIndex :type Integer))
  (Utilities|Casting|CastToBP_OverworldPlayerCharacter OtherActor)
  (CallFunction|OpenDoors))

(event EventBeginPlay
  (for _array_element (Components|GetChildrenComponents (Variables|Default|GetSocketParent) false)
    (Utilities|Array|AddUnique (Variables|Default|GetSockets) _array_element)))

(fn ConstructionScript)

(fn ShutDoors
  (for _array_element (Collision|GetOverlappingActors (Variables|Default|GetPlayerCheck) "/Game/RPG/DungeonGeneration/BP_Door.BP_Door_C" :!class /Script/Engine.PrimitiveComponent)
    (bind _asbp_door (Utilities|Casting|CastToBP_Door _array_element))
    (Default|ShutDoor _asbp_door)))

(fn OpenDoors
  (for _array_element (Collision|GetOverlappingActors (Variables|Default|GetPlayerCheck) "/Game/RPG/DungeonGeneration/BP_Door.BP_Door_C" :!class /Script/Engine.PrimitiveComponent)
    (bind _asbp_door (Utilities|Casting|CastToBP_Door _array_element))
    (Default|OpenDoor _asbp_door)))