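; Dungeon door actor that slides its mesh between open and shut positions and adjusts the overworld player's camera around the doorway.
; BeginPlay caches both positions and opens the door; Open and Shut timelines lerp from the current location, hiding the mesh once raised and showing it before lowering.
; Entering the box detaches the player's follow camera at a fixed rotation; leaving moves it to the Billboard and reattaches it to the boom.
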(event OnComponentBeginOverlap(Box)
  (params (OverlappedComponent :type Primitive%20Component%20Object%20Reference) (OtherActor :type Actor%20Object%20Reference) (OtherComp :type Primitive%20Component%20Object%20Reference) (OtherBodyIndex :type Integer) (bFromSweep :type Boolean) (SweepResult :type Hit%20Result%20Structure%20%28by%20ref%29))
  (bind _asbp_overworld_player_character (Utilities|Casting|CastToBP_OverworldPlayerCharacter OtherActor))
  (Transformation|DetachFromComponent (Variables|/Script/DevilInTheDungeon.DevilInTheDungeonCharacter|GetFollowCamera _asbp_overworld_player_character) "KeepWorld" "KeepRelative" "KeepWorld" true)
  (Transformation|SetWorldRotation (Variables|/Script/DevilInTheDungeon.DevilInTheDungeonCharacter|GetFollowCamera _asbp_overworld_player_character) "-10.000000,0.000000,0.000000" false false))

(event OnComponentEndOverlap(Box)
  (params (OverlappedComponent :type Primitive%20Component%20Object%20Reference) (OtherActor :type Actor%20Object%20Reference) (OtherComp :type Primitive%20Component%20Object%20Reference) (OtherBodyIndex :type Integer))
  (bind _asbp_overworld_player_character (Utilities|Casting|CastToBP_OverworldPlayerCharacter OtherActor))
  (Transformation|SetWorldLocation (Variables|/Script/DevilInTheDungeon.DevilInTheDungeonCharacter|GetFollowCamera _asbp_overworld_player_character) (Transformation|GetWorldLocation (Variables|/Game/RPG/Overworld/BP_OverworldPlayerCharacter.BP_OverworldPlayerCharacter_C|GetBillboard _asbp_overworld_player_character)) false false)
  (Transformation|AttachComponentToComponent (Variables|/Script/DevilInTheDungeon.DevilInTheDungeonCharacter|GetFollowCamera _asbp_overworld_player_character) (Variables|/Script/DevilInTheDungeon.DevilInTheDungeonCharacter|GetCameraBoom _asbp_overworld_player_character) "None" "KeepWorld" "KeepWorld" "KeepWorld" true)
  (Transformation|SetRelativeRotation (Variables|/Script/DevilInTheDungeon.DevilInTheDungeonCharacter|GetFollowCamera _asbp_overworld_player_character) "-10.000000,0.000000,0.000000" false false))

(event Custom|Shut%20Door
  (Rendering|SetVisibility (Variables|Default|GetDoor) true false)
  (bind _shut (Timeline|Shut PlayFromStart)
    (:Update
      (Transformation|SetWorldLocation (Variables|Default|GetDoor) (Math|Vector|Lerp(Vector) (Transformation|GetWorldLocation (Variables|Default|GetDoor)) (Variables|Default|GetDown) _shut) false false))))

(event Custom|Open%20Door
  (bind _shut (Timeline|Open PlayFromStart)
    (:Update
      (Transformation|SetWorldLocation (Variables|Default|GetDoor) (Math|Vector|Lerp(Vector) (Transformation|GetWorldLocation (Variables|Default|GetDoor)) (Variables|Default|GetUp) _shut) false false))
    (:Finished
      (Rendering|SetVisibility (Variables|Default|GetDoor) false false))))

(event EventBeginPlay
  (bind _door (Variables|Default|GetDoor))
  (bind _returnvalue (Transformation|GetWorldLocation _door))
  (bind (_x _y _z) (Math|Vector|BreakVector _returnvalue))
  (Variables|Default|SetDown _returnvalue)
  (Variables|Default|SetUp (Math|Vector|MakeVector _x _y (+ _z 4e+02)))
  (CallFunction|OpenDoor))

(event Collision|EventActorBeginOverlap
  (params (OtherActor :type Actor%20Object%20Reference)))

(event EventTick
  (params (DeltaSeconds :type Float%20%28single-precision%29)))

(fn ConstructionScript)