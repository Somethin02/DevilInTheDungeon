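; BP_4wayStart_Props is a dungeon generation room, apparently the four-way start room with props, built on a parent class.
; BeginPlay runs the parent logic, then clears the Locked flag.
; The RoomBounds overlap activates the overworld player character's CameraBoom on entry, with leftover debug prints, and deactivates it on exit.
; The construction script only calls the parent's.
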(event OnComponentBeginOverlap(RoomBounds)
  (params (OverlappedComponent :type Primitive%20Component%20Object%20Reference) (OtherActor :type Actor%20Object%20Reference) (OtherComp :type Primitive%20Component%20Object%20Reference) (OtherBodyIndex :type Integer) (bFromSweep :type Boolean) (SweepResult :type Hit%20Result%20Structure%20%28by%20ref%29))
  (bind _asbp_overworld_player_character (Utilities|Casting|CastToBP_OverworldPlayerCharacter OtherActor))
  (Development|PrintString "camera shid")
  (Components|Activation|Activate (Variables|/Script/DevilInTheDungeon.DevilInTheDungeonCharacter|GetCameraBoom _asbp_overworld_player_character) true)
  (Development|PrintString "camera shid"))

(event OnComponentEndOverlap(RoomBounds)
  (params (OverlappedComponent :type Primitive%20Component%20Object%20Reference) (OtherActor :type Actor%20Object%20Reference) (OtherComp :type Primitive%20Component%20Object%20Reference) (OtherBodyIndex :type Integer))
  (bind _asbp_overworld_player_character (Utilities|Casting|CastToBP_OverworldPlayerCharacter OtherActor))
  (Components|Activation|Deactivate (Variables|/Script/DevilInTheDungeon.DevilInTheDungeonCharacter|GetCameraBoom _asbp_overworld_player_character)))

(event EventBeginPlay
  (|CallParentFunction)
  (Variables|Default|SetLocked false))

(event Collision|EventActorBeginOverlap
  (params (OtherActor :type Actor%20Object%20Reference)))

(event EventTick
  (params (DeltaSeconds :type Float%20%28single-precision%29)))

(fn ConstructionScript
  (|CallParentFunction))