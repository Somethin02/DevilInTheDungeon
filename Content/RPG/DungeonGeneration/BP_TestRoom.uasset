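; BP_TestRoom is a test room actor for dungeon generation that collects its socket components at runtime.
; One frame after BeginPlay, it rebuilds RoomSockets from the valid direct children of its Plane component, then stores the total in SocketCount.
; Debug strings report the child count and each validity check, and the "current number of sockets" message actually prints the index returned by AddUnique.
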(event EventBeginPlay
  (bind _plane (Variables|Default|GetPlane))
  (bind _children (Components|GetChildrenComponents _plane false))
  (Utilities|FlowControl|DelayUntilNextFrame)
  (Development|PrintString (Utilities|String|ToString(Integer) (Utilities|Array|Length _children)) true true "(R=1.000000,G=0.000000,B=0.732790,A=1.000000)" 5e+01)
  (Utilities|Array|Clear (Variables|Default|GetRoom%20Sockets))
  (for _array_element _children
    (if (Utilities|IsValid _array_element)
      (Development|PrintString "kill me(true" true true "(R=0.000000,G=0.660000,B=1.000000,A=1.000000)" 2e+01)
      (bind _returnvalue (Utilities|Array|AddUnique (Variables|Default|GetRoom%20Sockets) _array_element))
      (Development|PrintString (Utilities|String|Append "current number of sockets" (Utilities|String|ToString(Integer) _returnvalue)) true true "(R=0.000000,G=0.660000,B=1.000000,A=1.000000)" 2e+01)
      (else
        (Development|PrintString "kill me(false" true true "(R=0.000000,G=0.660000,B=1.000000,A=1.000000)" 2e+01))))
  (Variables|Default|SetSocketCount (Utilities|Array|Length (Variables|Default|GetRoom%20Sockets))))

(event Collision|EventActorBeginOverlap
  (params (OtherActor :type Actor%20Object%20Reference)))

(event EventTick
  (params (DeltaSeconds :type Float%20%28single-precision%29)))

(fn ConstructionScript)