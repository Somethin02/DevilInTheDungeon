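; Base dungeon room that locks the player in for an enemy encounter and reopens once cleared.
; On BeginPlay it gathers its child socket components; when the player enters PlayerCheck while Locked, it shuts overlapping doors and has the spawn manager place enemies at marked locations.
; It derives a salted stream from the master seed, unused in these graphs.
; EnemyDeathCheck waits a tick, then unlocks and opens doors if no enemies overlap, otherwise prints one's name.
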(event OnComponentBeginOverlap(PlayerCheck)
  (params (OverlappedComponent :type Primitive%20Component%20Object%20Reference) (OtherActor :type Actor%20Object%20Reference) (OtherComp :type Primitive%20Component%20Object%20Reference) (OtherBodyIndex :type Integer) (bFromSweep :type Boolean) (SweepResult :type Hit%20Result%20Structure%20%28by%20ref%29))
  (Utilities|Casting|CastToBP_OverworldPlayerCharacter OtherActor)
  (if (Variables|Default|GetLocked)
    (CallFunction|ShutDoors)
    (CallFunction|SpawnEnemies)))

(event OnComponentEndOverlap(PlayerCheck)
  (params (OverlappedComponent :type Primitive%20Component%20Object%20Reference) (OtherActor :type Actor%20Object%20Reference) (OtherComp :type Primitive%20Component%20Object%20Reference) (OtherBodyIndex :type Integer)))

(event Custom|EnemyDeathCheck
  (bind _playercheck (Variables|Default|GetPlayerCheck))
  (bind _overlappingactors (Collision|GetOverlappingActors _playercheck "/Game/RPG/Overworld/BP_OverworldEnemy.BP_OverworldEnemy_C" :!class /Script/Engine.PrimitiveComponent))
  (Utilities|FlowControl|DelayUntilNextTick)
  (if (Utilities|Array|IsEmpty _overlappingactors)
    (CallFunction|OpenDoors)
    (else
      (Development|PrintString (Utilities|GetDisplayName (Utilities|Array|Get(acopy) _overlappingactors)) true true "(R=0.025430,G=1.000000,B=0.403703,A=1.000000)" 1e+01))))

(event Custom|Spawn%20Enemies
  (bind _asgi_rpg (Utilities|Casting|CastToGI_RPG (Game|GetGameInstance)))
  (Variables|Default|SetEnemySpawnSeed (Math|Random|MakeRandomStream (+ (Class|KismetMathLibrary|BreakRandomStream (Variables|/Game/GI_RPG.GI_RPG_C|GetMasterSeed _asgi_rpg)) (Variables|Default|GetEnemySpawnSalt))))
  (bind _returnvalue (Actor|GetActorOfClass "/Game/RPG/Overworld/BP_OverworldEnemySpawnManager.BP_OverworldEnemySpawnManager_C"))
  (Variables|Default|SetEnemyManager _returnvalue)
  (for _array_element (Components|GetChildrenComponents (Variables|Default|GetEnemySpawnLocations) false)
    (Default|SpawnEnemy (Variables|Default|GetEnemyManager) (Transformation|GetWorldTransform _array_element))))

(event EventBeginPlay
  (for _array_element (Components|GetChildrenComponents (Variables|Default|GetSocketParent) false)
    (Utilities|Array|AddUnique (Variables|Default|GetSockets) _array_element)))

(fn ConstructionScript)

(fn ShutDoors
  (for _array_element (Collision|GetOverlappingActors (Variables|Default|GetPlayerCheck) "/Game/RPG/DungeonGeneration/BP_Door.BP_Door_C" :!class /Script/Engine.PrimitiveComponent)
    (bind _asbp_door (Utilities|Casting|CastToBP_Door _array_element))
    (Default|ShutDoor _asbp_door)))

(fn OpenDoors
  (Variables|Default|SetLocked false)
  (for _array_element (Collision|GetOverlappingActors (Variables|Default|GetPlayerCheck) "/Game/RPG/DungeonGeneration/BP_Door.BP_Door_C" :!class /Script/Engine.PrimitiveComponent)
    (bind _asbp_door (Utilities|Casting|CastToBP_Door _array_element))
    (Default|OpenDoor _asbp_door)))