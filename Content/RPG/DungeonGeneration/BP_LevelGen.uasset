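; Procedural dungeon generator that builds a level at BeginPlay, using a random stream seeded from the game instance's master seed plus a salt.
; From a start room, it attaches connector rooms at socket arrows, destroying overlapping placements and retrying other candidates.
; Dead ends, walls and one exit, gated by room count and distance, close sockets.
; It spawns doors, enemies, chests and the next-level trigger, then notifies the enemy spawn manager.
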(event Custom|Spawn%20Exit
  (Variables|Default|SetCurrentRoomToSpawn (.OutItem (Utilities|Array|RandomFromStream (Variables|Default|GetSpawnableFloorExitRooms) (Variables|Default|GetLevelGenSeed))))
  (Variables|Default|SetTarget%20Arrow (Utilities|Array|Get(acopy) (Variables|Default|GetTargetSockets)))
  (bind _returnvalue (Game|SpawnActorfromClass (Variables|Default|GetCurrentRoomToSpawn) (Transformation|GetWorldTransform (Variables|Default|GetTarget%20Arrow)) "AlwaysSpawn" "MultiplyWithRoot" 0 0))
  (CallFunction|AddOverlapRoomstoList _returnvalue)
  (if (Utilities|Array|IsNotEmpty (Variables|Default|GetOverlapList))
    (Utilities|Array|Clear (Variables|Default|GetOverlapList))
    (Actor|DestroyActor _returnvalue)
    (CallFunction|BlockOffExit)
    (else
      (Game|SpawnActorfromClass "/Game/RPG/DungeonGeneration/BP_NextLevelTrigger.BP_NextLevelTrigger_C" (Transformation|GetWorldTransform (Components|GetChildComponent (Variables|/Game/RPG/DungeonGeneration/BP_ParentRoom.BP_ParentRoom_C|GetLevelExitParent _returnvalue) 0)) "Undefined" "MultiplyWithRoot" 0 0)
      (CallFunction|SpawnDoor)
      (Utilities|Array|RemoveItem (Variables|Default|GetTargetSockets) (Variables|Default|GetTarget%20Arrow))
      (Variables|Default|SetExitSpawned true)
      (CallFunction|SpawnConnectorRoom))))

(event Custom|SpawnStartRoom
  (bind _returnvalue (Game|SpawnActorfromClass (.OutItem (Utilities|Array|RandomFromStream (Variables|Default|GetStarterRooms) (Variables|Default|GetLevelGenSeed))) (Math|Transform|MakeTransform "-500.000000,0.000000,0.000000" "0, 0, 0" "1.000000,1.000000,1.000000") "Undefined" "MultiplyWithRoot" 0 0))
  (Variables|Default|SetStartRoom _returnvalue)
  (Variables|Default|SetPreviouslySpawnedRoom _returnvalue)
  (Utilities|Array|AppendArray (Variables|Default|GetTargetSockets) (Components|GetChildrenComponents (Variables|/Game/RPG/DungeonGeneration/BP_ParentRoom.BP_ParentRoom_C|GetSocketParent (Variables|Default|GetPreviouslySpawnedRoom)) false))
  (Utilities|Array|AddUnique (Variables|Default|GetSpawnedRooms) _returnvalue))

(event Custom|Add%20overlap%20rooms%20to%20list
  (params (Spawned%20Room :type BP%20Parent%20Room%20Object%20Reference))
  (Utilities|IsValid Spawned%20Room
    (:Is%20Valid
      (for _array_element (Components|GetChildrenComponents (Variables|/Game/RPG/DungeonGeneration/BP_ParentRoom.BP_ParentRoom_C|GetCollisionParent Spawned%20Room) false)
        (bind _asbox_collision (Utilities|Casting|CastToBoxComponent _array_element))
        (Utilities|Array|AppendArray (Variables|Default|GetOverlapList) (Class|PrimitiveComponent|GetOverlappingComponents _asbox_collision))
        (for _array_element_2 (Class|PrimitiveComponent|GetOverlappingComponents _asbox_collision)
          (Development|PrintString (Utilities|GetObjectName _array_element_2)))))
    (:Is%20Not%20Valid
      (for _array_element_3 (Components|GetChildrenComponents (Variables|/Game/RPG/DungeonGeneration/BP_ParentRoom.BP_ParentRoom_C|GetCollisionParent (Variables|Default|GetPreviouslySpawnedRoom)) false)
        (bind _asbox_collision_2 (Utilities|Casting|CastToBoxComponent _array_element_3))
        (Utilities|Array|AppendArray (Variables|Default|GetOverlapList) (Class|PrimitiveComponent|GetOverlappingComponents _asbox_collision_2))
        (for _array_element_4 (Class|PrimitiveComponent|GetOverlappingComponents _asbox_collision_2)
          (Development|PrintString (Utilities|GetObjectName _array_element_4)))))))

(event Custom|SpawnConnectorRoom
  (bind _targetsockets (Variables|Default|GetTargetSockets))
  (bind _output (Utilities|Array|Get(acopy) _targetsockets))
  (if (Variables|Default|GetRetrying)
    (Variables|Default|SetCurrentRoomToSpawn (.OutItem (Utilities|Array|RandomFromStream (Variables|Default|GetSpawnableConnecterRooms) (Variables|Default|GetLevelGenSeed))) :!label _label)
    (Utilities|IsValid _output
      (:Is%20Valid
        (Variables|Default|SetTarget%20Arrow _output))
      (:Is%20Not%20Valid
        (Variables|Default|GetTarget%20Arrow
          (:then
            _)
          (:else))))
    (bind _currentroomtospawn (Variables|Default|GetCurrentRoomToSpawn)
      (:then
        (bind _returnvalue (Game|SpawnActorfromClass _currentroomtospawn (Transformation|GetWorldTransform (Variables|Default|GetTarget%20Arrow)) "AlwaysSpawn" "MultiplyWithRoot" 0 0))
        (bind _output_get (Variables|Default|SetPreviouslySpawnedRoom _returnvalue))
        (Variables|Default|SetPreviouslySpawnedRoomLocation (Transformation|GetActorLocation _output_get))
        (CallFunction|AddOverlapRoomstoList))
      (:else
        _))
    (if (Utilities|Array|IsNotEmpty (Variables|Default|GetOverlapList))
      (Variables|Default|SetRetrying true)
      (bind _previouslyspawnedroom (Variables|Default|GetPreviouslySpawnedRoom)
        (:then
          (Actor|DestroyActor _previouslyspawnedroom)
          (Utilities|Array|Clear (Variables|Default|GetOverlapList)))
        (:else
          _))
      (Utilities|Array|RemoveItem (Variables|Default|GetSpawnableConnecterRooms) (Variables|Default|GetCurrentRoomToSpawn))
      (Utilities|Array|AddUnique (Variables|Default|GetConnecterRoomsToRetry) (Variables|Default|GetCurrentRoomToSpawn))
      (if (Utilities|Array|IsEmpty (Variables|Default|GetSpawnableConnecterRooms))
        (Variables|Default|SetRetrying false)
        (CallFunction|SpawnDeadEnd)
        (else
          (CallFunction|SpawnConnectorRoom)))
      (else
        (Variables|Default|SetRetrying false)
        (Utilities|Array|Clear (Variables|Default|GetOverlapList))
        (bind _previouslyspawnedroom_2 (Variables|Default|GetPreviouslySpawnedRoom)
          (:then
            (Utilities|Array|AppendArray (Variables|Default|GetTargetSockets) (Components|GetChildrenComponents (Variables|/Game/RPG/DungeonGeneration/BP_ParentRoom.BP_ParentRoom_C|GetSocketParent _previouslyspawnedroom_2) false))
            (Utilities|Array|AddUnique (Variables|Default|GetSpawnedRooms) (Variables|Default|GetPreviouslySpawnedRoom)))
          (:else
            _))
        (Utilities|Array|RemoveItem (Variables|Default|GetSpawnableConnecterRooms) (Variables|Default|GetCurrentRoomToSpawn))
        (CallFunction|SpawnEnemies)
        (CallFunction|SpawnDoor)
        (Utilities|Array|RemoveItem (Variables|Default|GetTargetSockets) (Variables|Default|GetTarget%20Arrow))
        (if (Utilities|Array|IsEmpty (Variables|Default|GetConnecterRoomsToRetry))
          _
          (else
            (Utilities|Array|AppendArray (Variables|Default|GetSpawnableConnecterRooms) (Variables|Default|GetConnecterRoomsToRetry))
            (Utilities|Array|Clear (Variables|Default|GetConnecterRoomsToRetry))))
        (if (>= (Utilities|Array|Length (Variables|Default|GetSpawnedRooms)) (Variables|Default|GetMaxRoomCount))
          (CallFunction|SpawnDeadEnd)
          (else
            (Variables|Default|SetTarget%20Arrow 0)
            (CallFunction|SpawnConnectorRoom)))))
    (elif (or (>= (Utilities|Array|Length (Variables|Default|GetSpawnedRooms)) (Variables|Default|GetMaxRoomCount)) (Utilities|Array|IsEmpty (Variables|Default|GetSpawnableConnecterRooms)))
      (CallFunction|SpawnDeadEnd)
      (else
        (goto _label)))))

(event Custom|Spawn%20Door
  (Game|SpawnActorfromClass "/Game/RPG/DungeonGeneration/BP_Door.BP_Door_C" (Transformation|GetWorldTransform (Variables|Default|GetTarget%20Arrow)) "Undefined" "MultiplyWithRoot" 0 0))

(event Custom|SpawnDeadEnd
  (Variables|Default|GetTarget%20Arrow
    (:then
      (if (not (Variables|Default|GetExitSpawned)) :!label _label
        (if (and (>= (Utilities|Array|Length (Variables|Default|GetSpawnedRooms)) (Variables|Default|GetMinimumRoomsBeforeExit)) (> (Math|Vector|Distance(Vector) (Transformation|GetActorLocation (Variables|Default|GetStartRoom)) (Variables|Default|GetPreviouslySpawnedRoomLocation)) (Variables|Default|GetMinimumDistanceToSpawnExit)))
          (CallFunction|SpawnExit)
          (else
            (if (Utilities|Array|IsNotEmpty (Variables|Default|GetSpawnableDeadEndRooms)) :!label _label_2
              (Variables|Default|SetCurrentRoomToSpawn (.OutItem (Utilities|Array|RandomFromStream (Variables|Default|GetSpawnableDeadEndRooms) (Variables|Default|GetLevelGenSeed))))
              (Variables|Default|SetTarget%20Arrow (Utilities|Array|Get(acopy) (Variables|Default|GetTargetSockets)))
              (bind _currentroomtospawn (Variables|Default|GetCurrentRoomToSpawn)
                (:then
                  (bind _returnvalue (Game|SpawnActorfromClass _currentroomtospawn (Transformation|GetWorldTransform (Variables|Default|GetTarget%20Arrow)) "AlwaysSpawn" "MultiplyWithRoot" 0 0))
                  (bind _output_get (Variables|Default|SetPreviouslySpawnedRoom _returnvalue))
                  (Variables|Default|SetPreviouslySpawnedRoomLocation (Transformation|GetActorLocation _output_get))
                  (CallFunction|AddOverlapRoomstoList)
                  (if (Utilities|Array|IsNotEmpty (Variables|Default|GetOverlapList))
                    (bind _previouslyspawnedroom (Variables|Default|GetPreviouslySpawnedRoom :!label _label_3)
                      (:then
                        (Actor|DestroyActor _previouslyspawnedroom)
                        (Utilities|Array|Clear (Variables|Default|GetOverlapList)))
                      (:else
                        _))
                    (Utilities|Array|RemoveItem (Variables|Default|GetSpawnableDeadEndRooms) (Variables|Default|GetCurrentRoomToSpawn))
                    (Utilities|Array|AddUnique (Variables|Default|GetConnecterRoomsToRetry) (Variables|Default|GetCurrentRoomToSpawn))
                    (if (Utilities|Array|IsEmpty (Variables|Default|GetSpawnableDeadEndRooms))
                      (CallFunction|BlockOffExit)
                      (Variables|Default|SetTarget%20Arrow 0)
                      (else
                        (CallFunction|SpawnDeadEnd)))
                    (else
                      (Development|PrintString "Hello")
                      (Utilities|Array|Clear (Variables|Default|GetOverlapList))
                      (Utilities|Array|RemoveItem (Variables|Default|GetSpawnableDeadEndRooms) (Variables|Default|GetCurrentRoomToSpawn))
                      (CallFunction|SpawnEnemies)
                      (CallFunction|SpawnChests)
                      (CallFunction|SpawnDoor)
                      (Utilities|Array|RemoveItem (Variables|Default|GetTargetSockets) (Variables|Default|GetTarget%20Arrow))
                      (Variables|Default|SetTarget%20Arrow 0)
                      (if (Utilities|Array|IsEmpty (Variables|Default|GetConnecterRoomsToRetry))
                        _
                        (else
                          (Utilities|Array|AppendArray (Variables|Default|GetSpawnableConnecterRooms) (Variables|Default|GetConnecterRoomsToRetry))
                          (Utilities|Array|Clear (Variables|Default|GetConnecterRoomsToRetry))))
                      (if (>= (Utilities|Array|Length (Variables|Default|GetSpawnedRooms)) (Variables|Default|GetMaxRoomCount))
                        (CallFunction|BlockOffExit)
                        (CallFunction|SpawnDeadEnd)
                        (else
                          (Variables|Default|SetTarget%20Arrow 0)
                          (Development|PrintString (Utilities|String|ToString(Integer) (Utilities|Array|Length (Variables|Default|GetSpawnedRooms))))
                          (if (Utilities|Array|IsNotEmpty (Variables|Default|GetTargetSockets))
                            (CallFunction|SpawnConnectorRoom)))))))
                (:else
                  (goto _label_3)))
              (else
                (Variables|Default|SetTarget%20Arrow (Utilities|Array|Get(acopy) (Variables|Default|GetTargetSockets)))
                (CallFunction|BlockOffExit)))))
        (else
          (goto _label_2))))
    (:else
      (if (Utilities|Array|IsEmpty (Variables|Default|GetTargetSockets))
        ;[0.15 0.15 0.15 0.5] Finished Generating Successfully
        (Utilities|FlowControl|DoOnce false
          (:Completed
            (bind _returnvalue_2 (Actor|GetActorOfClass "/Game/RPG/Overworld/BP_OverworldEnemySpawnManager.BP_OverworldEnemySpawnManager_C"))
            (Default|LevelFinished _returnvalue_2)))
        (else
          (goto _label))))))

(event Custom|Block%20off%20exit
  (Variables|Default|SetRetrying false)
  (bind _target_arrow (Variables|Default|GetTarget%20Arrow)
    (:then
      (Development|PrintString (Utilities|String|ToString(Integer) (Utilities|Array|Length (Variables|Default|GetTargetSockets))))
      (Game|SpawnActorfromClass "/Game/RPG/DungeonGeneration/BP_Wall.BP_Wall_C" (Transformation|GetWorldTransform _target_arrow) "Undefined" "MultiplyWithRoot" 0 0)
      (Utilities|Array|RemoveItem (Variables|Default|GetTargetSockets) (Variables|Default|GetTarget%20Arrow))
      (Utilities|Array|AppendArray (Variables|Default|GetSpawnableConnecterRooms) (Variables|Default|GetConnecterRoomsToRetry))
      (Utilities|FlowControl|DelayUntilNextFrame)
      (CallFunction|SpawnConnectorRoom))
    (:else)))

(event Custom|Spawn%20Enemies
  (bind _previouslyspawnedroom (Variables|Default|GetPreviouslySpawnedRoom)
    (:then
      (if (not (Utilities|Array|IsEmpty (Components|GetChildrenComponents (Variables|/Game/RPG/DungeonGeneration/BP_ParentRoom.BP_ParentRoom_C|GetEnemySpawnLocations _previouslyspawnedroom) false)))
        (for _array_element (Components|GetChildrenComponents (Variables|/Game/RPG/DungeonGeneration/BP_ParentRoom.BP_ParentRoom_C|GetEnemySpawnLocations _previouslyspawnedroom) false)
          (Game|SpawnActorfromClass "/Game/RPG/Overworld/BP_OverworldEnemySpawner.BP_OverworldEnemySpawner_C" (Transformation|GetWorldTransform _array_element) "Undefined" "MultiplyWithRoot" 0 0))))
    (:else)))

(event Custom|Spawn%20Chests
  (for _array_element (Components|GetChildrenComponents (Variables|/Game/RPG/DungeonGeneration/BP_ParentRoom.BP_ParentRoom_C|GetChestsParent (Variables|Default|GetPreviouslySpawnedRoom)) false)
    (Game|SpawnActorfromClass "/Game/RPG/BP_Chest.BP_Chest_C" (Transformation|GetWorldTransform _array_element) "Undefined" "MultiplyWithRoot" 0 0)))

(event EventBeginPlay
  (bind _asgi_rpg (Utilities|Casting|CastToGI_RPG (Game|GetGameInstance))
    (:then
      (Variables|Default|SetLevelGenSeed (Math|Random|MakeRandomStream (+ (Class|KismetMathLibrary|BreakRandomStream (Variables|/Game/GI_RPG.GI_RPG_C|GetMasterSeed _asgi_rpg)) (Variables|Default|GetLevelGenSalt))))
      (CallFunction|SpawnStartRoom)
      (CallFunction|SpawnConnectorRoom))
    (:CastFailed
      (Development|PrintString "oops, no game instance found"))))

(fn ConstructionScript)