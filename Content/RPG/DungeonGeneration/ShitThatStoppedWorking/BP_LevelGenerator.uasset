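; Unfinished socket-based procedural dungeon generator, with debug prints throughout and its seeded main loop disconnected from any event.
; From a start room, it moves random pre-placed connector rooms so an arrow-component socket meets an open socket, rotated 180 degrees.
; Bounds overlaps destroy the room and queue it for retry; successful placements add open sockets.
; Dead-end placement logic is unwired, exit-room spawning is empty, and CleanUp destroys leftover rooms.
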(event Custom|SpawnDeadEnd
  (if (Utilities|Array|IsNotEmpty (Variables|Default|GetDeadEndRooms))
    _
    (else
      _))
  (Development|PrintString "NoDeadEnds or ConnectingRooms")
  (Variables|Default|SetDoneGeneratingLevel true))

(event Custom|SpawnConnectorRoom
  (bind _targetroomsockets (Variables|Default|GetTargetRoomSockets))
  (bind _connectorroomstoretryspawning (Variables|Default|GetConnectorRoomsToRetrySpawning))
  (bind _targetroomsockets_2 (Variables|Default|GetTargetRoomSockets))
  (if (Utilities|Array|IsNotEmpty (Variables|Default|GetConnectorRooms))
    (bind _output_get (Variables|Default|SetIncomingSocketRoomSpawn (.OutItem (Utilities|Array|RandomFromStream (Variables|Default|GetConnectorRooms) (Variables|Default|GetLevelGenSeed)))))
    (CallFunction|GetSocketWorldLocations _output_get)
    (Utilities|Array|RemoveItem (Variables|Default|GetConnectorRooms) _output_get)
    (Variables|Default|SetIncomingSocket (Utilities|Array|Get(acopy) _targetroomsockets_2))
    (Development|PrintString (Utilities|String|Append "Incoming room has this many doors " (Utilities|String|ToString(Integer) (Utilities|Array|Length _targetroomsockets_2))))
    (Utilities|Array|RemoveIndex _targetroomsockets_2)
    (Development|PrintString (Utilities|String|Append "room sockets after removal " (Utilities|String|ToString(Integer) (Utilities|Array|Length (Variables|Default|GetTargetRoomSockets)))) true true "(R=1.000000,G=0.058759,B=0.037749,A=1.000000)" 2e+01)
    (bind _roomspawntransform (CallFunction|CalculateRoomSpawnTransform))
    (Rendering|Debug|DrawDebugString "0, 0, 0" (Utilities|String|ToString(Vector) (.location (Variables|Default|GetTargetSocket))) 0 "(R=1.000000,G=0.000000,B=0.097472,A=1.000000)" 1e+04)
    (Transformation|SetActorTransform (Variables|Default|GetIncomingSocketRoomSpawn) _roomspawntransform)
    (bind _outcomponents (Class|KismetSystemLibrary|ComponentOverlapComponents (Variables|/Game/RPG/DungeonGeneration/ShitThatStoppedWorking/BP_TestRoom.BP_TestRoom_C|GetRoomBounds (Variables|Default|GetIncomingSocketRoomSpawn)) _roomspawntransform (Variables|Default|GetObject%20Types) "/Game/RPG/DungeonGeneration/ShitThatStoppedWorking/BP_TestRoom.BP_TestRoom_C"))
    (if (> (Utilities|Array|Length _outcomponents) 0)
      (Development|PrintString "actor destroyed" true true "(R=0.000000,G=0.660000,B=1.000000,A=1.000000)" 5.0)
      (Actor|DestroyActor (Variables|Default|GetIncomingSocketRoomSpawn))
      (Utilities|Array|AddUnique (Variables|Default|GetConnectorRoomsToRetrySpawning) (Variables|Default|GetIncomingSocketRoomSpawn))
      (else
        (bind _output_get_2 (Variables|Default|SetTargetRoom (Variables|Default|GetIncomingSocketRoomSpawn)))
        (Utilities|Array|AddUnique (Variables|Default|GetListOfSpawnedRooms) _output_get_2)
        (CallFunction|GetSocketWorldLocations _output_get_2)
        (Development|PrintString (Utilities|String|Append "Number of sockets in target room " (Utilities|String|ToString(Integer) (Utilities|Array|Length _targetroomsockets))) true true "(R=0.000000,G=0.660000,B=1.000000,A=1.000000)" 2e+01)
        (for _array_element _targetroomsockets
          (if (not (== (Variables|Default|GetIncomingSocket) _array_element))
            (Utilities|Array|AddUnique (Variables|Default|GetOpen%20Sockets) _array_element)))
        (Utilities|Array|AppendArray (Variables|Default|GetConnectorRooms) _connectorroomstoretryspawning)
        (Utilities|Array|Clear _connectorroomstoretryspawning)
        (Development|PrintString "room placed" true true "(R=0.000000,G=0.660000,B=1.000000,A=1.000000)" 5.0)
        (Development|PrintString (Utilities|String|Append "Length after placing room: " (Utilities|String|ToString(Integer) (Utilities|Array|Length (Variables|Default|GetOpen%20Sockets)))) true true "(R=0.000000,G=0.660000,B=1.000000,A=1.000000)" 2e+01)))
    (else
      (Development|PrintString "NoConnectingRooms"))))

(event Custom|SpawnExitRoom)

(event Custom|SpawnStartRoom
  (bind _returnvalue (Game|SpawnActorfromClass "/Game/RPG/DungeonGeneration/ShitThatStoppedWorking/BP_TestRoom.BP_TestRoom_C" (Math|Transform|MakeTransform "0, 0, 0" "0, 0, 0" "1.000000,1.000000,1.000000") "Undefined" "MultiplyWithRoot" 0 0))
  (Utilities|Array|AddUnique (Variables|Default|GetListOfSpawnedRooms) _returnvalue)
  (bind _output_get (Variables|Default|SetTargetRoom _returnvalue))
  (CallFunction|GetSocketWorldLocations _output_get)
  (bind _output_get_2 (Variables|Default|SetOpen%20Sockets (Variables|Default|GetTargetRoomSockets)))
  (Variables|Default|SetDoneGeneratingLevel (Utilities|Array|IsEmpty _output_get_2)))

(event Custom|CleanUp
  (for _array_element (Variables|Default|GetConnectorRooms)
    (Actor|DestroyActor _array_element))
  (for _array_element_2 (Variables|Default|GetDeadEndRooms)
    (Actor|DestroyActor _array_element_2)))

(event EventBeginPlay)

(event Collision|EventActorBeginOverlap
  (params (OtherActor :type Actor%20Object%20Reference)))

(event EventTick
  (params (DeltaSeconds :type Float%20%28single-precision%29)))

(fn ConstructionScript)

(fn CalculateRoomSpawnTransform
  (bind _targetsocket (Variables|Default|GetTargetSocket))
  (bind (_location _rotation _scale) (Math|Transform|BreakTransform _targetsocket))
  (return (Math|Transform|ComposeTransforms (Math|Transform|MakeRelativeTransform (Variables|Default|GetDefaultTransform) (Variables|Default|GetIncomingSocket)) (Math|Transform|MakeTransform _location (Math|Rotator|MakeRotator 0.0 0.0 (+ (.Yaw (Math|Rotator|BreakRotator _rotation)) 1.8e+02)) _scale))))

(fn GetSocketWorldLocations
  (params (Room :type BP%20Test%20Room%20Object%20Reference))
  (bind _output_get (LocalVariables|SetRooms Room))
  (for _array_element (Actor|GetComponentsByClass _output_get "/Script/Engine.ArrowComponent")
    (Utilities|Array|AddUnique (Variables|Default|GetTargetRoomSockets) (Transformation|GetWorldTransform _array_element)))
  (return))