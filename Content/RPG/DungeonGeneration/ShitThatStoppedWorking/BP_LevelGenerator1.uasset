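; Experimental dungeon level generator that spawns a start room and snaps a randomly picked connector room to a socket, with debug prints throughout.
; Socket transforms drive a relative-transform calculation that positions and yaws the connector against the target room.
; A bounds overlap check either destroys the connector and queues it for retry, or records it and its open sockets.
; The seeded startup chain is disconnected, and TargetSocket is never assigned here.
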(event Custom|SpawnConnectorRoom
  (bind _targetroomsockets (Variables|Default|GetTargetRoomSockets))
  (bind _connectorroomstoretryspawning (Variables|Default|GetConnectorRoomsToRetrySpawning))
  (bind _targetroomsockets_2 (Variables|Default|GetTargetRoomSockets))
  (bind _output_get (Variables|Default|SetIncomingSocketRoomSpawn (.OutItem (Utilities|Array|RandomFromStream (Variables|Default|GetConnectorRooms) (Variables|Default|GetLevelGenSeed)))))
  (Development|PrintString (Utilities|String|Append "Socket Count" (Utilities|String|ToString(Integer) (Variables|/Game/RPG/DungeonGeneration/ShitThatStoppedWorking/BP_TestRoom.BP_TestRoom_C|GetSocketCount _output_get))) true true "(R=0.385286,G=0.000000,B=1.000000,A=1.000000)" 2e+01)
  (CallFunction|GetSocketTransforms (Variables|/Game/RPG/DungeonGeneration/ShitThatStoppedWorking/BP_TestRoom.BP_TestRoom_C|GetRoom%20Sockets _output_get))
  (Utilities|Array|RemoveItem (Variables|Default|GetConnectorRooms) _output_get)
  (Variables|Default|SetIncomingSocket (Utilities|Array|Get(acopy) _targetroomsockets_2))
  (Development|PrintString (Utilities|String|Append "Incoming room has this many doors " (Utilities|String|ToString(Integer) (Utilities|Array|Length _targetroomsockets_2))))
  (Utilities|Array|RemoveIndex _targetroomsockets_2)
  (bind _roomspawntransform (CallFunction|CalculateRoomSpawnTransform))
  (Transformation|SetActorTransform (Variables|Default|GetIncomingSocketRoomSpawn) _roomspawntransform)
  (Development|PrintString "Hello")
  (bind _outcomponents (Class|KismetSystemLibrary|ComponentOverlapComponents (Variables|/Game/RPG/DungeonGeneration/ShitThatStoppedWorking/BP_TestRoom.BP_TestRoom_C|GetRoomBounds (Variables|Default|GetIncomingSocketRoomSpawn)) _roomspawntransform (Variables|Default|GetObject%20Types) "/Game/RPG/DungeonGeneration/ShitThatStoppedWorking/BP_TestRoom.BP_TestRoom_C"))
  (if (> (Utilities|Array|Length _outcomponents) 0)
    (Development|PrintString "actor destroyed" true true "(R=0.000000,G=0.660000,B=1.000000,A=1.000000)" 5.0)
    (Actor|DestroyActor (Variables|Default|GetIncomingSocketRoomSpawn))
    (Utilities|Array|AddUnique (Variables|Default|GetConnectorRoomsToRetrySpawning) (Variables|Default|GetIncomingSocketRoomSpawn))
    (else
      (Development|PrintString (Utilities|String|Append "Number of sockets in target room " (Utilities|String|ToString(Integer) (Utilities|Array|Length _targetroomsockets))) true true "(R=0.000000,G=0.660000,B=1.000000,A=1.000000)" 2e+01)
      (for _array_element _targetroomsockets
        (if (not (== (Variables|Default|GetIncomingSocket) _array_element))
          (Utilities|Array|AddUnique (Variables|Default|GetOpen%20Sockets) _array_element)))
      (bind _output_get_2 (Variables|Default|SetTargetRoom (Variables|Default|GetIncomingSocketRoomSpawn)))
      (Utilities|Array|AddUnique (Variables|Default|GetListOfSpawnedRooms) _output_get_2)
      (Utilities|Array|AppendArray (Variables|Default|GetConnectorRooms) _connectorroomstoretryspawning)
      (Utilities|Array|Clear _connectorroomstoretryspawning)
      (Development|PrintString "room placed" true true "(R=0.000000,G=0.660000,B=1.000000,A=1.000000)" 5.0)
      (Development|PrintString (Utilities|String|Append "Length after placing room: " (Utilities|String|ToString(Integer) (Utilities|Array|Length (Variables|Default|GetOpen%20Sockets)))) true true "(R=0.000000,G=0.660000,B=1.000000,A=1.000000)" 2e+01))))

(event Custom|SpawnStartRoom
  (bind _returnvalue (Game|SpawnActorfromClass "/Game/RPG/DungeonGeneration/ShitThatStoppedWorking/BP_TestRoom.BP_TestRoom_C" (Math|Transform|MakeTransform "0, 0, 0" "0, 0, 0" "1.000000,1.000000,1.000000") "Undefined" "MultiplyWithRoot" 0 0))
  (Utilities|Array|AddUnique (Variables|Default|GetListOfSpawnedRooms) _returnvalue)
  (bind _output_get (Variables|Default|SetTargetRoom _returnvalue))
  (CallFunction|GetSocketTransforms (Variables|/Game/RPG/DungeonGeneration/ShitThatStoppedWorking/BP_TestRoom.BP_TestRoom_C|GetRoom%20Sockets _output_get))
  (bind _output_get_2 (Variables|Default|SetOpen%20Sockets (Variables|Default|GetTargetRoomSockets)))
  (Variables|Default|SetDoneGeneratingLevel (Utilities|Array|IsEmpty _output_get_2)))

(event EventBeginPlay)

(event Collision|EventActorBeginOverlap
  (params (OtherActor :type Actor%20Object%20Reference)))

(event EventTick
  (params (DeltaSeconds :type Float%20%28single-precision%29)))

(fn ConstructionScript)

(fn CalculateRoomSpawnTransform
  (bind _incomingsocketroomspawn (Variables|Default|GetIncomingSocketRoomSpawn))
  (bind _incomingsocket (Variables|Default|GetIncomingSocket))
  (bind _defaultsceneroot (Variables|/Game/RPG/DungeonGeneration/ShitThatStoppedWorking/BP_TestRoom.BP_TestRoom_C|GetDefaultSceneRoot _incomingsocketroomspawn))
  (bind _returnvalue (Transformation|GetWorldTransform _defaultsceneroot))
  (bind _returnvalue_2 (Math|Transform|MakeRelativeTransform _returnvalue _incomingsocket))
  (return (Math|Transform|MakeTransform (+ (.location (Variables|Default|GetTargetSocket)) (.location _returnvalue_2)) (Math|Rotator|CombineRotators (.rotation _returnvalue_2) (Math|Rotator|MakeRotator 0.0 0.0 (+ (.yaw (.rotation (Math|Transform|MakeRelativeTransform (Transformation|GetWorldTransform (Variables|/Game/RPG/DungeonGeneration/ShitThatStoppedWorking/BP_TestRoom.BP_TestRoom_C|GetDefaultSceneRoot (Variables|Default|GetTargetRoom))) (Variables|Default|GetTargetSocket)))) 1.8e+02))) "1.000000,1.000000,1.000000")))

(fn GetSocketTransforms
  (params (RoomSockets :type Array%20of%20Scene%20Component%20Object%20References))
  (Utilities|Array|Clear (Variables|Default|GetTargetRoomSockets))
  (for _array_element RoomSockets
    (Utilities|Array|AddUnique (Variables|Default|GetTargetRoomSockets) (Transformation|GetWorldTransform _array_element)))
  (return))