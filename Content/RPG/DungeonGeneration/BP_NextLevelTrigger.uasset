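; BP_NextLevelTrigger is a dungeon exit trigger that sends the player on to the next level.
; When the overworld player character overlaps its Box, it rebuilds the GI_RPG game instance's MasterSeed stream from the initial seed plus a fixed offset.
; It then calls OpenNextLevel on the first player's BP_BattleCharacterController, so each level starts from a new, deterministic seed.
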(event OnComponentBeginOverlap(Box)
  (params (OverlappedComponent :type Primitive%20Component%20Object%20Reference) (OtherActor :type Actor%20Object%20Reference) (OtherComp :type Primitive%20Component%20Object%20Reference) (OtherBodyIndex :type Integer) (bFromSweep :type Boolean) (SweepResult :type Hit%20Result%20Structure%20%28by%20ref%29))
  (Utilities|Casting|CastToBP_OverworldPlayerCharacter OtherActor)
  (bind _asbp_battle_character_controller (Utilities|Casting|CastToBP_BattleCharacterController (Game|GetPlayerController 0)))
  (bind _asgi_rpg (Utilities|Casting|CastToGI_RPG (Game|GetGameInstance)))
  (Variables|/Game/GI_RPG.GI_RPG_C|SetMasterSeed _asgi_rpg (Math|Random|MakeRandomStream (+ (Class|KismetMathLibrary|BreakRandomStream (Variables|/Game/GI_RPG.GI_RPG_C|GetMasterSeed _asgi_rpg)) 10)))
  (Default|OpenNextLevel _asbp_battle_character_controller))

(event EventBeginPlay)

(event Collision|EventActorBeginOverlap
  (params (OtherActor :type Actor%20Object%20Reference)))

(event EventTick
  (params (DeltaSeconds :type Float%20%28single-precision%29)))

(fn ConstructionScript)