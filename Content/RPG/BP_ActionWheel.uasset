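; RPG action wheel actor that shows a rotating 3D ring of ability categories available to its AbilityOwner.
; On BeginPlay it builds slots from non-empty owned ability lists (attack, elemental spells, items, spirit, tactics) and spawns labeled meshes.
; RotateWheel plays a timeline that lerps yaw, placing meshes by sine/cosine, then updates the wrapped index.
; SelectActionSlot sends that category's abilities to the HUD once, guarded by SlotSelected.
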(event Custom|SpawnActionBlocks
  (bind _wheelpivot (Variables|Default|GetWheelPivot))
  (bind _returnvalue (Transformation|GetRelativeTransform _wheelpivot))
  ;[0.15 0.15 0.15 0.5] Something with how the blocks are spawned. The index appears fine, but visually, the blocks don't all match their abilities
  (for _array_element (Variables|Default|GetActionSlots)
    (bind _returnvalue_2 (AddComponent|AddStaticMeshComponent true (Math|Transform|MakeTransform (Math|Vector|MakeVector (+ (.x (.location _returnvalue)) 1e+02) (.y (.location _returnvalue)) (.z (.location _returnvalue))) (.rotation _returnvalue) (.scale _returnvalue))))
    (Components|StaticMesh|SetStaticMesh _returnvalue_2 (.Mesh (Utilities|Struct|BreakS_ActionSlot _array_element)))
    (Transformation|AttachComponentToComponent _returnvalue_2 (Variables|Default|GetWheelPivot) "None" "KeepRelative" "KeepWorld" "KeepRelative" true)
    (Class|PrimitiveComponent|SetConstraintMode _returnvalue_2 "XZPlane")
    (Utilities|Array|AddUnique (Variables|Default|GetSpawnedMeshes) _returnvalue_2)
    (bind _returnvalue_3 (AddComponent|AddTextRenderComponent false (Math|Transform|MakeTransform (Math|Vector|MakeVector (+ (.x (.location (Transformation|GetRelativeTransform _returnvalue_2))) -1.2e+02) (+ (.y (.location (Transformation|GetRelativeTransform _returnvalue_2))) 7e+01) (.z (.location (Transformation|GetRelativeTransform _returnvalue_2)))) (.rotation (Transformation|GetRelativeTransform _returnvalue_2)) (.scale (Transformation|GetRelativeTransform _returnvalue_2)))))
    (Rendering|Components|TextRender|SetText _returnvalue_3 (.ActionName (Utilities|Struct|BreakS_ActionSlot _array_element)))
    (Rendering|Components|TextRender|SetTextRenderColor _returnvalue_3 (Variables|Default|GetTextColor))
    (Transformation|AttachComponentToComponent _returnvalue_3 _returnvalue_2 "None" "KeepRelative" "KeepRelative" "KeepRelative" true)
    (CallFunction|CalculateMeshPositions)))

(event Custom|CheckOwnedAbilities
  (bind _abilityowner (Variables|Default|GetAbilityOwner))
  (bind _ac_abilitysystem (Variables|/Game/RPG/BP_TurnBasedActor.BP_TurnBasedActor_C|GetAC_AbilitySystem _abilityowner))
  (if (Utilities|Array|IsNotEmpty (Variables|/Game/RPG/AC_AbilitySystem.AC_AbilitySystem_C|GetOwnedAttackAbilities _ac_abilitysystem))
    (bind _output_get (Variables|Default|SetNewSlot (Utilities|Struct|MakeS_ActionSlot "Attack" "/Game/Meshes/AttackCube.AttackCube" "NewEnumerator0" "NewEnumerator3")))
    (Utilities|Array|AddUnique (Variables|Default|GetActionSlots) _output_get))
  (if (Utilities|Array|IsNotEmpty (Variables|/Game/RPG/AC_AbilitySystem.AC_AbilitySystem_C|GetOwnedFireAbilities _ac_abilitysystem))
    (bind _output_get_2 (Variables|Default|SetNewSlot (Utilities|Struct|MakeS_ActionSlot "Fire" "/Game/AssetPacks/Fantastic_Dungeon_Pack/meshes/props/small_deco/SM_PROP_book_dungeon_01.SM_PROP_book_dungeon_01" "NewEnumerator1" "NewEnumerator0")))
    (Utilities|Array|AddUnique (Variables|Default|GetActionSlots) _output_get_2))
  (if (Utilities|Array|IsNotEmpty (Variables|/Game/RPG/AC_AbilitySystem.AC_AbilitySystem_C|GetOwnedLightningAbilities _ac_abilitysystem))
    (bind _output_get_3 (Variables|Default|SetNewSlot (Utilities|Struct|MakeS_ActionSlot "Lightning" "/Game/AssetPacks/Fantastic_Dungeon_Pack/meshes/props/small_deco/SM_PROP_book_dungeon_03.SM_PROP_book_dungeon_03" "NewEnumerator1" "NewEnumerator2")))
    (Utilities|Array|AddUnique (Variables|Default|GetActionSlots) _output_get_3))
  (if (Utilities|Array|IsNotEmpty (Variables|/Game/RPG/AC_AbilitySystem.AC_AbilitySystem_C|GetOwnedWaterAbilities _ac_abilitysystem))
    (bind _output_get_4 (Variables|Default|SetNewSlot (Utilities|Struct|MakeS_ActionSlot "Water" "/Game/AssetPacks/Fantastic_Dungeon_Pack/meshes/props/small_deco/SM_PROP_book_dungeon_02.SM_PROP_book_dungeon_02" "NewEnumerator1" "NewEnumerator1")))
    (Utilities|Array|AddUnique (Variables|Default|GetActionSlots) _output_get_4))
  (if (Utilities|Array|IsNotEmpty (Variables|/Game/RPG/AC_AbilitySystem.AC_AbilitySystem_C|GetOwnedItemAbilities _ac_abilitysystem))
    (bind _output_get_5 (Variables|Default|SetNewSlot (Utilities|Struct|MakeS_ActionSlot "Items" "/Game/Meshes/ItemCube.ItemCube" "NewEnumerator2" "NewEnumerator3")))
    (Utilities|Array|AddUnique (Variables|Default|GetActionSlots) _output_get_5))
  (if (Utilities|Array|IsNotEmpty (Variables|/Game/RPG/AC_AbilitySystem.AC_AbilitySystem_C|GetOwnedSpiritAbilities _ac_abilitysystem))
    (bind _output_get_6 (Variables|Default|SetNewSlot (Utilities|Struct|MakeS_ActionSlot "Spirit" "/Game/Meshes/SpiritCube.SpiritCube" "NewEnumerator3" "NewEnumerator3")))
    (Utilities|Array|AddUnique (Variables|Default|GetActionSlots) _output_get_6))
  (if (Utilities|Array|IsNotEmpty (Variables|/Game/RPG/AC_AbilitySystem.AC_AbilitySystem_C|GetOwnedTacticsAbilities _ac_abilitysystem))
    (bind _output_get_7 (Variables|Default|SetNewSlot (Utilities|Struct|MakeS_ActionSlot "Tactics" "/Game/Meshes/TacticsCube.TacticsCube" "NewEnumerator4" "NewEnumerator3")))
    (Utilities|Array|AddUnique (Variables|Default|GetActionSlots) _output_get_7)))

(event Custom|RotateWheel
  (params (Direction :type Integer))
  (if (not (Variables|Default|GetSpinning))
    (Variables|Default|SetSpinning true)
    (bind _output_get (Variables|Default|SetStartRot (Variables|Default|GetCurrentWheelRot)))
    (Variables|Default|SetNewRot (Math|Rotator|MakeRotator (.roll _output_get) (.pitch _output_get) (+ (.yaw _output_get) (* (/ 360 (Utilities|Array|Length (Variables|Default|GetSpawnedMeshes))) Direction))))
    (bind _newtrack_0 (Timeline|Spin PlayFromStart)
      (:Update
        (Variables|Default|SetCurrentWheelRot (Math|Rotator|Lerp(Rotator) (Variables|Default|GetStartRot) (Variables|Default|GetNewRot) _newtrack_0))
        (CallFunction|CalculateMeshPositions))
      (:Finished
        (Variables|Default|SetSpinning false)
        (CallFunction|UpdateIndex Direction)))))

(event Custom|UpdateIndex
  (params (Direction :type Integer))
  (bind _spawnedmeshes (Variables|Default|GetSpawnedMeshes))
  (bind _returnvalue (Utilities|Array|Length _spawnedmeshes))
  (bind _returnvalue_2 (- _returnvalue 1))
  (if (Variables|Default|GetSpinning)
    (Development|PrintString "fucky wucki\\")
    (else
      (if (> (+ (Variables|Default|GetCurrentIndex) (* 1 Direction)) _returnvalue_2)
        (Variables|Default|SetCurrentIndex 0)
        (elif (< (+ (Variables|Default|GetCurrentIndex) (* 1 Direction)) 0)
          (Variables|Default|SetCurrentIndex _returnvalue_2)
          (else
            (Variables|Default|SetCurrentIndex (+ (Variables|Default|GetCurrentIndex) (* 1 Direction))))))
      (Development|PrintString (Utilities|String|ToString(Integer) (Variables|Default|GetCurrentIndex))))))

(event Custom|SelectActionSlot
  (bind _abilityowner (Variables|Default|GetAbilityOwner))
  (bind _actionslots (Variables|Default|GetActionSlots))
  (bind _currentindex (Variables|Default|GetCurrentIndex))
  (bind _output (Utilities|Array|Get(acopy) _actionslots _currentindex))
  (bind _ac_abilitysystem (Variables|/Game/RPG/BP_TurnBasedActor.BP_TurnBasedActor_C|GetAC_AbilitySystem _abilityowner))
  (bind (_actionname _mesh _abilitytype _element) (Utilities|Struct|BreakS_ActionSlot _output))
  (if (not (Variables|Default|GetbSlotSelected))
    (Variables|Default|SetbSlotSelected true)
    (Development|PrintText _actionname)
    (switch Utilities|FlowControl|Switch|SwitchonE_Ability _abilitytype
      (:NewEnumerator0
        (for _array_element (Variables|/Game/RPG/AC_AbilitySystem.AC_AbilitySystem_C|GetOwnedAttackAbilities _ac_abilitysystem)
          (Default|SetPlayerInfo (Variables|Default|GetHUDReference) (Variables|Default|GetAbilityOwner) _array_element)))
      (:NewEnumerator1
        (switch Utilities|FlowControl|Switch|SwitchonE_Elements _element
          (:NewEnumerator0
            (for _array_element_2 (Variables|/Game/RPG/AC_AbilitySystem.AC_AbilitySystem_C|GetOwnedFireAbilities _ac_abilitysystem)
              (Default|SetPlayerInfo (Variables|Default|GetHUDReference) (Variables|Default|GetAbilityOwner) _array_element_2)))
          (:NewEnumerator1
            (for _array_element_3 (Variables|/Game/RPG/AC_AbilitySystem.AC_AbilitySystem_C|GetOwnedWaterAbilities _ac_abilitysystem)
              (Default|SetPlayerInfo (Variables|Default|GetHUDReference) (Variables|Default|GetAbilityOwner) _array_element_3)))
          (:NewEnumerator2
            (for _array_element_4 (Variables|/Game/RPG/AC_AbilitySystem.AC_AbilitySystem_C|GetOwnedLightningAbilities _ac_abilitysystem)
              (Default|SetPlayerInfo (Variables|Default|GetHUDReference) (Variables|Default|GetAbilityOwner) _array_element_4)))))
      (:NewEnumerator2
        (for _array_element_5 (Variables|/Game/RPG/AC_AbilitySystem.AC_AbilitySystem_C|GetOwnedItemAbilities _ac_abilitysystem)
          (Default|SetPlayerInfo (Variables|Default|GetHUDReference) (Variables|Default|GetAbilityOwner) _array_element_5)))
      (:NewEnumerator3
        (for _array_element_6 (Variables|/Game/RPG/AC_AbilitySystem.AC_AbilitySystem_C|GetOwnedSpiritAbilities _ac_abilitysystem)
          (Default|SetPlayerInfo (Variables|Default|GetHUDReference) (Variables|Default|GetAbilityOwner) _array_element_6)))
      (:NewEnumerator4
        (for _array_element_7 (Variables|/Game/RPG/AC_AbilitySystem.AC_AbilitySystem_C|GetOwnedTacticsAbilities _ac_abilitysystem)
          (Default|SetPlayerInfo (Variables|Default|GetHUDReference) (Variables|Default|GetAbilityOwner) _array_element_7))))))

(event EventBeginPlay
  (CallFunction|CheckOwnedAbilities)
  (CallFunction|SpawnActionBlocks))

(fn ConstructionScript)

(fn CalculateMeshPositions
  (bind _spawnedmeshes (Variables|Default|GetSpawnedMeshes))
  (for (_array_element _array_index) _spawnedmeshes
    (Transformation|SetRelativeLocation _array_element (Math|Vector|MakeVector (* (Math|Trig|Cos(Radians) (Math|Trig|DegreesToRadians (Math|Conversions|ToFloat(Integer) (+ (* _array_index (/ 360 (Utilities|Array|Length _spawnedmeshes))) (.yaw (Variables|Default|GetCurrentWheelRot)))))) 1e+02) (* (Math|Trig|Sin(Radians) (Math|Trig|DegreesToRadians (Math|Conversions|ToFloat(Integer) (+ (* _array_index (/ 360 (Utilities|Array|Length _spawnedmeshes))) (.yaw (Variables|Default|GetCurrentWheelRot)))))) 1e+02) 0.0) false false)))