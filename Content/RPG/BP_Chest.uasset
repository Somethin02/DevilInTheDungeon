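; BP_Chest is an overworld chest that opens when the player walks into it and drops an upgrade.
; A sphere overlap by BP_OverworldPlayerCharacter plays a timeline that rotates the lid mesh, guarded by an Open flag.
; When the timeline finishes, it sets Open and spawns a BP_Upgrade at the item spawn point, then launches it with that point's transform.
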(event OnComponentBeginOverlap(Sphere)
  (params (OverlappedComponent :type Primitive%20Component%20Object%20Reference) (OtherActor :type Actor%20Object%20Reference) (OtherComp :type Primitive%20Component%20Object%20Reference) (OtherBodyIndex :type Integer) (bFromSweep :type Boolean) (SweepResult :type Hit%20Result%20Structure%20%28by%20ref%29))
  (Utilities|Casting|CastToBP_OverworldPlayerCharacter OtherActor)
  (CallFunction|OpenChest))

(event Custom|OpenChest
  (if (not (Variables|Default|GetbOpen))
    (bind _open (Timeline|Timeline PlayFromStart)
      (:Update
        (Transformation|SetRelativeRotation (Variables|Default|GetStaticMesh1) (Math|Rotator|MakeRotator (Math|Float|Lerp 0.0 -95.0 _open) 0.0 0.0) false false))
      (:Finished
        (Variables|Default|SetbOpen true)
        (CallFunction|SpawnDrop)))))

(event Custom|SpawnDrop
  (bind _itemspawnpoint (Variables|Default|GetItemSpawnPoint))
  (bind _returnvalue (Transformation|GetWorldTransform _itemspawnpoint))
  (bind _returnvalue_2 (Game|SpawnActorfromClass "/Game/RPG/BP_Upgrade.BP_Upgrade_C" _returnvalue "Undefined" "MultiplyWithRoot" 0 0))
  (Default|Launch _returnvalue_2 _returnvalue))

(event EventBeginPlay)

(event Collision|EventActorBeginOverlap
  (params (OtherActor :type Actor%20Object%20Reference)))

(event EventTick
  (params (DeltaSeconds :type Float%20%28single-precision%29)))

(fn ConstructionScript)