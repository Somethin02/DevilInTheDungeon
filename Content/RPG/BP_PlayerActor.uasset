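; Player actor for a turn-based RPG, granting Wait, Attack and Heal abilities through its ability system component on BeginPlay.
; When its turn becomes active, it spawns an action wheel above the mesh or unhides the existing one.
; GiveXp derives level from an XP curve, and LevelUp applies an HP effect based on the current maximum.
; AddGrimoire grants every spell in a grimoire as an ability.
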(event Custom|SpawnWheel
  (bind _mesh (Variables|Character|GetMesh))
  (bind _returnvalue (Transformation|GetWorldTransform _mesh))
  (Utilities|IsValid (Variables|Default|GetAction%20Wheel)
    (:Is%20Valid
      (Rendering|SetActorHiddenInGame (Variables|Default|GetAction%20Wheel) false))
    (:Is%20Not%20Valid
      (bind _returnvalue_2 (Game|SpawnActorfromClass "/Game/RPG/BP_ActionWheel.BP_ActionWheel_C" (Math|Transform|MakeTransform (Math|Vector|MakeVector (.x (.location _returnvalue)) (.y (.location _returnvalue)) (+ (.z (.location _returnvalue)) 3e+02)) (.rotation _returnvalue) (.scale _returnvalue)) "Undefined" "MultiplyWithRoot" 0 self (Variables|Default|GetHUD) 0))
      (Variables|Default|SetAction%20Wheel _returnvalue_2))))

(event EventBeginPlay
  (bind _ac_abilitysystem (Variables|Default|GetAC_AbilitySystem))
  (|CallParentFunction)
  (Default|GiveAbility _ac_abilitysystem "/Game/RPG/GA_Wait.GA_Wait_C")
  (Default|GiveAbility _ac_abilitysystem "/Game/RPG/GA_Attack.GA_Attack_C")
  (Default|GiveAbility _ac_abilitysystem "/Game/RPG/GA_Heal.GA_Heal_C")
  (CallFunction|LevelUp 1))

(event Collision|EventActorBeginOverlap
  (params (OtherActor :type Actor%20Object%20Reference))
  (|CallParentFunction OtherActor) ; This node is disabled and will not be called.\nDrag off pins to build functionality.
)

(event EventTick
  (params (DeltaSeconds :type Float%20%28single-precision%29))
  (|CallParentFunction DeltaSeconds) ; This node is disabled and will not be called.\nDrag off pins to build functionality.
)

(event EventSetTurnActive
  (params (IsActive? :type Boolean))
  (bind _mesh (Variables|Character|GetMesh))
  (bind _returnvalue (Transformation|GetWorldTransform _mesh))
  (if IsActive?
    (Utilities|IsValid (Variables|Default|GetAction%20Wheel)
      (:Is%20Valid
        (Rendering|SetActorHiddenInGame (Variables|Default|GetAction%20Wheel) false))
      (:Is%20Not%20Valid
        (bind _returnvalue_2 (Game|SpawnActorfromClass "/Game/RPG/BP_ActionWheel.BP_ActionWheel_C" (Math|Transform|MakeTransform (Math|Vector|MakeVector (.x (.location _returnvalue)) (.y (.location _returnvalue)) (+ (.z (.location _returnvalue)) 3e+02)) (.rotation _returnvalue) (.scale _returnvalue)) "Undefined" "MultiplyWithRoot" 0 self (Variables|Default|GetHUD) 0))
        (Variables|Default|SetAction%20Wheel _returnvalue_2)))))

(fn ConstructionScript
  (|CallParentFunction))

(fn GiveXp
  (params (XP :type Integer))
  (bind _output_get (Variables|Default|SetTotalXP (+ XP (Variables|Default|GetTotalXP))))
  (if (> (Math|Float|Floor (Math|Curves|GetFloatValue (Variables|Default|GetXPCurve) (Math|Conversions|ToFloat(Integer) _output_get))) (Variables|Default|GetLevel))
    (CallFunction|LevelUp (Math|Float|Floor (Math|Curves|GetFloatValue (Variables|Default|GetXPCurve) (Math|Conversions|ToFloat(Integer) _output_get))))))

(fn LevelUp
  (params (NewLevel :type Integer))
  (bind _ac_abilitysystem (Variables|Default|GetAC_AbilitySystem))
  (Variables|Default|SetLevel NewLevel)
  (bind _maxvalue_withmods_ (Default|GetAttributeMaximum _ac_abilitysystem "HP"))
  (Development|PrintString (Utilities|String|ToString(Float) (+ _maxvalue_withmods_ 5.0)) true true "(R=0.251335,G=1.000000,B=0.220595,A=1.000000)")
  (Default|ApplyEffecttoSelf _ac_abilitysystem "NewEnumerator0" "HP" "NewEnumerator2" "NewEnumerator3" (+ _maxvalue_withmods_ 5.0))
  (bind _maxvalue_withmods__2 (Default|GetAttributeMaximum _ac_abilitysystem "HP"))
  (Development|PrintString (Utilities|String|Append "Level Up!" " HP: " (Utilities|String|ToString(Float) _maxvalue_withmods__2))))

(fn AddGrimoire
  (params (Grimoire :type BP%20Grimoire%20Object%20Reference))
  (for _array_element (Variables|/Game/RPG/BP_Grimoire.BP_Grimoire_C|GetSpells Grimoire)
    (Default|GiveAbility (Variables|Default|GetAC_AbilitySystem) _array_element))
  (Actor|DestroyActor))