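; BP_TurnBasedActor is an actor for the RPG turn-based battle that shows turn, targeting and value-change feedback on its mesh.
; Turn and target events swap the mesh overlay material between outline, thick outline and none.
; Losing target restores the turn outline if ACAbilitySystem says it is still this actor's turn.
; Value changes spawn BP_DamageNumbers at the mesh transform, and a getter exposes ACAbilitySystem.
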(event Custom|DisplayValueChange
  (params (Difference :type Integer))
  (bind _mesh (Variables|Character|GetMesh))
  (bind _returnvalue (Transformation|GetWorldTransform _mesh))
  (Game|SpawnActorfromClass "/Game/RPG/UI/BP_DamageNumbers.BP_DamageNumbers_C" (Math|Transform|MakeTransform (Math|Vector|MakeVector (.x (.location _returnvalue)) (.y (.location _returnvalue)) (.z (.location _returnvalue))) (.rotation _returnvalue) (.scale _returnvalue)) "Undefined" "MultiplyWithRoot" 0 Difference 0))

(event EventBeginPlay)

(event Collision|EventActorBeginOverlap
  (params (OtherActor :type Actor%20Object%20Reference)))

(event EventTick
  (params (DeltaSeconds :type Float%20%28single-precision%29)))

(event EventSetTurnActive
  (params (IsActive? :type Boolean))
  (bind _mesh (Variables|Character|GetMesh))
  (if IsActive?
    (Rendering|Material|SetOverlayMaterial _mesh "/Game/Materials/M_Outline.M_Outline" :!class /Script/Engine.MeshComponent)
    (else
      (Rendering|Material|SetOverlayMaterial _mesh 0 :!class /Script/Engine.MeshComponent))))

(event EventSetTargeted
  (params (IsTargeted :type Boolean))
  (bind _mesh (Variables|Character|GetMesh))
  (if IsTargeted
    (Rendering|Material|SetOverlayMaterial _mesh "/Game/Materials/MI_ThickOutline.MI_ThickOutline" :!class /Script/Engine.MeshComponent)
    (elif (Variables|/Game/RPG/AC_AbilitySystem.AC_AbilitySystem_C|GetIsTurn (Variables|Default|GetAC_AbilitySystem))
      (Rendering|Material|SetOverlayMaterial _mesh "/Game/Materials/M_Outline.M_Outline" :!class /Script/Engine.MeshComponent)
      (else
        (Rendering|Material|SetOverlayMaterial _mesh 0 :!class /Script/Engine.MeshComponent)))))

(fn ConstructionScript)

(fn GetTurnBasedComponent
  (return (Variables|Default|GetAC_AbilitySystem)))