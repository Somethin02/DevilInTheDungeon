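; BP_EnemyActor is an enemy in the RPG battle that shows its stats on a widget and attacks on its turn.
; On BeginPlay it fills W_EnemyStats with attack, defense and HP percent from its ability system attributes, and DisplayValueChange refreshes the HP percent.
; When the ability system signals TurnStarted, it targets a random active party member from BP_BattleCharacterController and activates GA_Attack, skipping selection.
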(event TurnStarted(AC_AbilitySystem)
  (bind _ac_abilitysystem (Variables|Default|GetAC_AbilitySystem))
  (bind _asbp_battle_character_controller (Utilities|Casting|CastToBP_BattleCharacterController (Game|GetPlayerController 0)))
  (Variables|/Game/RPG/AC_AbilitySystem.AC_AbilitySystem_C|SetTargetActor _ac_abilitysystem (.OutItem (Utilities|Array|Random (Variables|/Game/RPG/BP_BattleCharacterController.BP_BattleCharacterController_C|GetActiveParty _asbp_battle_character_controller))))
  (Default|ActivateSingleAbility _ac_abilitysystem "/Game/RPG/Battle/Abilities/GA_Attack.GA_Attack_C" true))

(event EventBeginPlay
  (bind _ac_abilitysystem (Variables|Default|GetAC_AbilitySystem))
  (|CallParentFunction)
  (bind _asw_enemy_stats (Utilities|Casting|CastToW_EnemyStats (UserInterface|GetWidget (Variables|Default|GetWidget))))
  (bind _currentvalue_withmods_ (Default|GetAttributeCurrent _ac_abilitysystem "ATK"))
  (Variables|/Game/RPG/UI/W_EnemyStats.W_EnemyStats_C|SetAttackPower _asw_enemy_stats (Math|Float|Truncate _currentvalue_withmods_))
  (bind _currentvalue_withmods__2 (Default|GetAttributeCurrent _ac_abilitysystem "DEF"))
  (Variables|/Game/RPG/UI/W_EnemyStats.W_EnemyStats_C|SetDefPower _asw_enemy_stats (Math|Float|Truncate _currentvalue_withmods__2))
  (bind _currentvalue_withmods__3 (Default|GetAttributeCurrent _ac_abilitysystem "HP"))
  (bind _maxvalue_withmods_ (Default|GetAttributeMaximum _ac_abilitysystem "HP"))
  (Variables|/Game/RPG/UI/W_EnemyStats.W_EnemyStats_C|SetHPPercent _asw_enemy_stats (/ _currentvalue_withmods__3 _maxvalue_withmods_)))

(event Collision|EventActorBeginOverlap
  (params (OtherActor :type Actor%20Object%20Reference))
  (|CallParentFunction OtherActor) ; This node is disabled and will not be called.\nDrag off pins to build functionality.
)

(event EventTick
  (params (DeltaSeconds :type Float%20%28single-precision%29))
  (|CallParentFunction DeltaSeconds) ; This node is disabled and will not be called.\nDrag off pins to build functionality.
)

(event EventDisplayValueChange
  (params (Difference :type Integer))
  (bind _ac_abilitysystem (Variables|Default|GetAC_AbilitySystem))
  (bind _asw_enemy_stats (Utilities|Casting|CastToW_EnemyStats (UserInterface|GetWidget (Variables|Default|GetWidget))))
  (bind _currentvalue_withmods_ (Default|GetAttributeCurrent _ac_abilitysystem "HP"))
  (bind _maxvalue_withmods_ (Default|GetAttributeMaximum _ac_abilitysystem "HP"))
  (Variables|/Game/RPG/UI/W_EnemyStats.W_EnemyStats_C|SetHPPercent _asw_enemy_stats (/ _currentvalue_withmods_ _maxvalue_withmods_)))

(fn ConstructionScript
  (|CallParentFunction))