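; Possessable turn-based RPG battle arena that runs a fight between the active party and an enemy encounter.
; On start it positions the party, spawns up to five enemies through chained async class loads, then cycles turns via each character's turn-based component.
; HUD-chosen ability actors handle target selection through debug-key input alongside the player's action wheel.
; Kill events bank XP and end battle, repossessing the overworld character, or open MainMenu when the party falls.
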(event Custom|StartBattle
  (params (ReturnCharacter :type Pawn%20Object%20Reference) (EnemyPositions :type Data%20Table%20Object%20Reference) (PlayerAdvantage :type Boolean) (EnemyAdvantage :type Boolean))
  (Variables|Default|SetPlayer%20Advantage PlayerAdvantage)
  (Variables|Default|SetEnemy%20Advantage EnemyAdvantage)
  (Variables|Default|SetEnemy%20Positions EnemyPositions)
  (Variables|Default|SetReturnCharacter ReturnCharacter)
  (Variables|Default|SetTurnOrderIndex 0)
  (Variables|Default|SetStopBattle false)
  (Rendering|SetActorHiddenInGame false)
  (CallFunction|MovePartytoBattlePositions)
  (CallFunction|SpawnEnemies))

(event Custom|MovePartyToBattlePositions
  (bind _asbp_battle_character_controller (Utilities|Casting|CastToBP_BattleCharacterController (Game|GetPlayerController 0)))
  (bind _output_get (Variables|Default|SetPlayerController _asbp_battle_character_controller))
  (for (_array_element _array_index) (Variables|/Game/RPG/BP_BattleCharacterController.BP_BattleCharacterController_C|GetActiveParty _output_get)
    (Utilities|IsValid _array_element
      (:Is%20Valid
        (Transformation|SetActorTransform _array_element (Transformation|GetWorldTransform (Utilities|Array|Get(acopy) (Utilities|Array|MakeArray (Variables|Default|GetPlayer1) (Variables|Default|GetPlayer2) (Variables|Default|GetPlayer3)) _array_index)))
        (Rendering|SetActorHiddenInGame _array_element false)
        (bind _component (Class|BPITurnBasedCombat|GetTurnBasedComponent(Message) _array_element))
        (EventDispatchers|AssignActorKilled _component (delegate Custom|ActorKilled_Event_0))
        (bind _asbp_player_actor (Utilities|Casting|CastToBP_PlayerActor _array_element))
        (Variables|/Game/RPG/Battle/PlayerPartyMembers/BP_PlayerActor.BP_PlayerActor_C|SetHUD _asbp_player_actor (Variables|Default|GetBattleHUD)))
      (:Is%20Not%20Valid
        (Development|PrintString "no character to move")))))

(event Custom|ActorKilled_Event_0
  (params (Actor :type Actor%20Object%20Reference))
  (CallFunction|LoseBattle))

(event Custom|SpawnEnemies
  (bind _asbp_battle_character_controller (Utilities|Casting|CastToBP_BattleCharacterController (Game|GetPlayerController 0)))
  (Variables|Default|SetEncounter (Variables|/Game/RPG/BP_BattleCharacterController.BP_BattleCharacterController_C|GetEnemyLayout _asbp_battle_character_controller))
  (bind _class (Utilities|AsyncLoadClassAsset (.Enemy1 (Utilities|Struct|BreakS_BasicEncounter (Variables|Default|GetEncounter))))
    (:Completed
      (bind _asactor (Utilities|Casting|CastToActorClass _class))
      (bind _returnvalue (Game|SpawnActorfromClass _asactor (Transformation|GetWorldTransform (Variables|Default|GetEnemy1)) "AlwaysSpawn" "MultiplyWithRoot" 0 0))
      (Utilities|Array|AddUnique (Variables|Default|GetEnemyParty) _returnvalue)
      (CallFunction|SetNewPartyMemberTarget _returnvalue)
      (bind _class_2 (Utilities|AsyncLoadClassAsset (.Enemy2 (Utilities|Struct|BreakS_BasicEncounter (Variables|Default|GetEncounter))))
        (:Completed
          (bind _asactor_2 (Utilities|Casting|CastToActorClass _class_2)
            (:then
              (bind _returnvalue_2 (Game|SpawnActorfromClass _asactor_2 (Transformation|GetWorldTransform (Variables|Default|GetEnemy2)) "AlwaysSpawn" "MultiplyWithRoot" 0 0))
              (Utilities|Array|AddUnique (Variables|Default|GetEnemyParty) _returnvalue_2)
              (CallFunction|SetNewPartyMemberTarget _returnvalue_2)
              (bind _class_3 (Utilities|AsyncLoadClassAsset (.Enemy3 (Utilities|Struct|BreakS_BasicEncounter (Variables|Default|GetEncounter))))
                (:Completed
                  (bind _asactor_3 (Utilities|Casting|CastToActorClass _class_3)
                    (:then
                      (bind _returnvalue_3 (Game|SpawnActorfromClass _asactor_3 (Transformation|GetWorldTransform (Variables|Default|GetEnemy3)) "AlwaysSpawn" "MultiplyWithRoot" 0 0))
                      (Utilities|Array|AddUnique (Variables|Default|GetEnemyParty) _returnvalue_3)
                      (CallFunction|SetNewPartyMemberTarget _returnvalue_3)
                      (bind _class_4 (Utilities|AsyncLoadClassAsset (.Enemy4 (Utilities|Struct|BreakS_BasicEncounter (Variables|Default|GetEncounter))))
                        (:Completed
                          (bind _asactor_4 (Utilities|Casting|CastToActorClass _class_4)
                            (:then
                              (bind _returnvalue_4 (Game|SpawnActorfromClass _asactor_4 (Transformation|GetWorldTransform (Variables|Default|GetEnemy4)) "AlwaysSpawn" "MultiplyWithRoot" 0 0))
                              (Utilities|Array|AddUnique (Variables|Default|GetEnemyParty) _returnvalue_4)
                              (CallFunction|SetNewPartyMemberTarget _returnvalue_4)
                              (bind _class_5 (Utilities|AsyncLoadClassAsset (.Enemy5 (Utilities|Struct|BreakS_BasicEncounter (Variables|Default|GetEncounter))))
                                (:Completed
                                  (bind _asactor_5 (Utilities|Casting|CastToActorClass _class_5)
                                    (:then
                                      (bind _returnvalue_5 (Game|SpawnActorfromClass _asactor_5 (Transformation|GetWorldTransform (Variables|Default|GetEnemy5)) "AlwaysSpawn" "MultiplyWithRoot" 0 0))
                                      (Utilities|Array|AddUnique (Variables|Default|GetEnemyParty) _returnvalue_5)
                                      (CallFunction|SetNewPartyMemberTarget _returnvalue_5))
                                    (:CastFailed
                                      _)))))
                            (:CastFailed
                              _)))))
                    (:CastFailed
                      _)))))
            (:CastFailed
              _))
          (CallFunction|SetTurnOrder)
          (CallFunction|NextCharacter)
          (for _array_element (Variables|Default|GetEnemyParty)
            (bind _component (Class|BPITurnBasedCombat|GetTurnBasedComponent(Message) _array_element))
            (EventDispatchers|AssignActorKilled _component (delegate Custom|ActorKilled_Event))))))))

(event Custom|NextCharacter
  (bind _returnvalue (Game|GetPlayerController 0))
  (Utilities|FlowControl|DelayUntilNextFrame)
  (if (Variables|Default|GetStopBattle)
    (Development|PrintString "Battle is OVER")
    (else
      (bind _targetedactor (Variables|Default|GetTargetedActor)
        (:then
          (Class|BPITurnBasedCombat|SetTargeted(Message) _targetedactor false))
        (:else
          _))
      (if (>= (Variables|Default|GetTurnOrderIndex) (Utilities|Array|Length (Variables|Default|GetTurnOrderActors)))
        (Variables|Default|SetTurnOrderIndex 0)
        (CallFunction|SetTurnOrder)
        (CallFunction|NextCharacter)
        (else
          (Utilities|IsValid (Utilities|Array|Get(acopy) (Variables|Default|GetTurnOrderActors) (Variables|Default|GetTurnOrderIndex))
            (:Is%20Valid
              (bind _component (Class|BPITurnBasedCombat|GetTurnBasedComponent(Message) (Utilities|Array|Get(acopy) (Variables|Default|GetTurnOrderActors) (Variables|Default|GetTurnOrderIndex))))
              (bind _currentvalue_withmods_ (Default|GetAttributeCurrent _component "HP"))
              (if (> _currentvalue_withmods_ 0.0)
                (Class|BPITurnBasedCombat|SetTurnActive(Message) (Variables|Default|GetActiveCharacter) false)
                (bind _output_get (Variables|Default|SetActiveCharacter (Utilities|Array|Get(acopy) (Variables|Default|GetTurnOrderActors) (Variables|Default|GetTurnOrderIndex))))
                (Class|BPITurnBasedCombat|SetTurnActive(Message) _output_get true)
                (Math|Integer|IncrementInt (Variables|Default|GetTurnOrderIndex)
                  (:%20%20
                    (bind _component_2 (Class|BPITurnBasedCombat|GetTurnBasedComponent(Message) (Variables|Default|GetActiveCharacter)))
                    (EventDispatchers|BindEventtoTurnEnded _component_2 (delegate Custom|TurnEndEvent))
                    (Default|StartTurn _component_2)
                    (bind _output_get_2 (Variables|Default|SetPlayersTurn (Utilities|Array|ContainsItem (Variables|/Game/RPG/BP_BattleCharacterController.BP_BattleCharacterController_C|GetActiveParty (Variables|Default|GetPlayerController)) (Variables|Default|GetActiveCharacter))))
                    (if _output_get_2
                      (EventDispatchers|BindEventtoAbilityChosen (Variables|Default|GetBattleHUD) (delegate Custom|AbilityChosen_Event))
                      (Input|SetInputModeGameandUI _returnvalue (Variables|Default|GetBattleHUD) "DoNotLock" true false)
                      (Variables|/Script/Engine.PlayerController|SetbShowMouseCursor _returnvalue true))))
                (else
                  (Development|PrintString "dead" :!label _label)
                  (Math|Integer|IncrementInt (Variables|Default|GetTurnOrderIndex)
                    (:%20%20
                      (CallFunction|NextCharacter))))))
            (:Is%20Not%20Valid
              (goto _label))))))))

(event Custom|TurnEndEvent
  (Development|PrintString "turn end vent")
  (Utilities|FlowControl|DelayUntilNextTick)
  (CallFunction|NextCharacter))

(event Custom|SetPlayerMenu
  (bind _returnvalue (Game|GetPlayerController 0))
  (bind _battlehud (Variables|Default|GetBattleHUD))
  (Default|SetPlayerInfo _battlehud (Variables|Default|GetActiveCharacter))
  (EventDispatchers|BindEventtoAbilityChosen (Variables|Default|GetBattleHUD) (delegate Custom|AbilityChosen_Event))
  (Input|SetInputModeGameandUI _returnvalue _battlehud "DoNotLock" true false)
  (Variables|/Script/Engine.PlayerController|SetbShowMouseCursor _returnvalue true))

(event Custom|AbilityChosen_Event
  (params (Ability :type BP%20Turn%20Based%20Ability%20Object%20Reference))
  (bind _playercontroller (Variables|Default|GetPlayerController))
  (bind _activeparty (Variables|/Game/RPG/BP_BattleCharacterController.BP_BattleCharacterController_C|GetActiveParty _playercontroller))
  (EventDispatchers|UnbindEventfromAbilityChosen (Variables|Default|GetBattleHUD) (delegate Custom|AbilityChosen_Event))
  (Variables|/Script/Engine.PlayerController|SetbShowMouseCursor (Game|GetPlayerController 0) false)
  (bind _component (Class|BPITurnBasedCombat|GetTurnBasedComponent(Message) (Variables|Default|GetActiveCharacter)))
  (Variables|Default|SetOwnPartySelected (Utilities|Array|ContainsItem _activeparty (Variables|/Game/RPG/AC_AbilitySystem.AC_AbilitySystem_C|GetTargetActor _component)))
  (bind _output_get (Variables|Default|SetCurrentAbility Ability))
  (CallFunction|SetSelectionbyIndex (Math|Integer|SelectInt (Utilities|Array|FindItem _activeparty (Variables|/Game/RPG/AC_AbilitySystem.AC_AbilitySystem_C|GetTargetActor _component)) (Utilities|Array|FindItem (Variables|Default|GetEnemyParty) 0) (Utilities|Array|ContainsItem _activeparty (Variables|/Game/RPG/AC_AbilitySystem.AC_AbilitySystem_C|GetTargetActor _component))))
  (bind _output (Default|UpdateSelectedTarget _output_get (Variables|/Game/RPG/BP_BattleCharacterController.BP_BattleCharacterController_C|GetActiveParty (Variables|Default|GetPlayerController)) (Variables|Default|GetEnemyParty) (Variables|Default|GetTargetedActor)))
  (Utilities|IsValid _output
    (:Is%20Valid
      (CallFunction|SetNewSelectedTarget _output)
      (Default|ClearAbilities (Variables|Default|GetBattleHUD)))
    (:Is%20Not%20Valid
      (Development|PrintString "no target" true true "(R=0.000000,G=0.660000,B=1.000000,A=1.000000)" 5.0)
      (CallFunction|CancelAbility))))

(event Custom|CancelAbility
  (Actor|DestroyActor (stale Input|KeyboardEvents|DebugKeyBackspace _currentability))
  (Default|ClearAbilities (Variables|Default|GetBattleHUD))
  (bind _asbp_player_actor (Utilities|Casting|CastToBP_PlayerActor (Variables|Default|GetActiveCharacter)))
  (Default|SpawnWheel _asbp_player_actor))

(event Custom|ActorKilled_Event
  (params (Actor :type Actor%20Object%20Reference))
  (bind _enemyparty (Variables|Default|GetEnemyParty))
  (Development|PrintString (Utilities|GetDisplayName Actor) true true "(R=1.000000,G=0.000000,B=0.003492,A=1.000000)" 5e+01)
  (Utilities|Array|RemoveItem _enemyparty Actor)
  (bind _asbp_enemy_actor (Utilities|Casting|CastToBP_EnemyActor Actor))
  (CallFunction|AddXPtoAward (Variables|/Game/RPG/Battle/Enemies/BP_EnemyActor.BP_EnemyActor_C|GetXPOnDeath _asbp_enemy_actor))
  (Utilities|FlowControl|Delay 2.0)
  (Actor|DestroyActor Actor)
  (if (Utilities|Array|IsEmpty _enemyparty)
    (Development|PrintString "urdead" true true "(R=1.000000,G=0.000000,B=0.003492,A=1.000000)" 5e+01)
    (CallFunction|EndBattle)))

(event Custom|End%20Battle
  (Variables|Default|SetStopBattle true)
  (Utilities|FlowControl|Delay 3.0)
  (CallFunction|AwardXP)
  (Rendering|SetActorHiddenInGame true)
  (for _array_element (CallFunction|GetBattleCharacters)
    (Rendering|SetActorHiddenInGame _array_element true)
    (bind _component (Class|BPITurnBasedCombat|GetTurnBasedComponent(Message) _array_element))
    (EventDispatchers|UnbindallEventsfromTurnEnded _component)
    (Class|BPITurnBasedCombat|SetTurnActive(Message) _array_element false)
    (Class|BPITurnBasedCombat|SetTargeted(Message) _array_element false))
  (Pawn|Possess (Game|GetPlayerController 0) (Variables|Default|GetReturnCharacter))
  (Widget|RemovefromParent (Variables|Default|GetBattleHUD))
  (Default|Die (Variables|Default|GetReturnEnemy)))

(event EventPossessed
  (params (NewController :type Controller%20Object%20Reference))
  (bind _asbp_battle_character_controller (Utilities|Casting|CastToBP_BattleCharacterController (Game|GetPlayerController 0)))
  (CallFunction|StartBattle (Variables|/Game/RPG/BP_BattleCharacterController.BP_BattleCharacterController_C|GetAs%20BP%20Overworld%20Player%20Character _asbp_battle_character_controller) "/Game/RPG/Data/DataTables/DT_EnemyEncounters.DT_EnemyEncounters" false false)
  (Utilities|FlowControl|DoOnce false
    (:Completed
      (UserInterface|Viewport|AddtoViewport (Variables|Default|GetBattleHUD) 0))))

(event EventBeginPlay
  (Variables|Default|SetEnemyPositions (Utilities|Array|MakeArray (Variables|Default|GetEnemy1) (Variables|Default|GetEnemy2) (Variables|Default|GetEnemy3) (Variables|Default|GetEnemy4) (Variables|Default|GetEnemy5)))
  (bind _asbp_battle_character_controller (Utilities|Casting|CastToBP_BattleCharacterController (Game|GetPlayerController 0)))
  (Variables|Default|SetPlayerController _asbp_battle_character_controller)
  (bind _returnvalue (UserInterface|CreateWidget "/Game/RPG/UI/W_BattleHUD.W_BattleHUD_C"))
  (Variables|Default|SetBattleHUD _returnvalue))

(event EventUnpossessed
  (params (OldController :type Controller%20Object%20Reference))
  (Widget|RemovefromParent (Variables|Default|GetBattleHUD))
  (Variables|/Script/Engine.PlayerController|SetbShowMouseCursor (Game|GetPlayerController 0) false)
  (Utilities|FlowControl|DoOnce false) ; enters at Reset
)

(event Input|KeyboardEvents|DebugKeyUp
  (params (Key :type Key%20Structure) (ActionValue :type Input%20Action%20Value%20Structure))
  (:Pressed
    (if (Variables|Default|GetPlayersTurn)
      (Variables|Default|GetCurrentAbility
        (:then
          (bind _output (Default|SelectOtherParty (Variables|Default|GetCurrentAbility) (Variables|/Game/RPG/BP_BattleCharacterController.BP_BattleCharacterController_C|GetActiveParty (Variables|Default|GetPlayerController)) (Variables|Default|GetEnemyParty) (Variables|Default|GetTargetedActor)))
          (CallFunction|SetNewSelectedTarget _output))
        (:else)))))

(event Input|KeyboardEvents|DebugKeyDown
  (params (Key :type Key%20Structure) (ActionValue :type Input%20Action%20Value%20Structure))
  (:Pressed
    (if (Variables|Default|GetPlayersTurn)
      (Variables|Default|GetCurrentAbility
        (:then
          (bind _output (Default|SelectOtherParty (Variables|Default|GetCurrentAbility) (Variables|/Game/RPG/BP_BattleCharacterController.BP_BattleCharacterController_C|GetActiveParty (Variables|Default|GetPlayerController)) (Variables|Default|GetEnemyParty) (Variables|Default|GetTargetedActor)))
          (CallFunction|SetNewSelectedTarget _output))
        (:else)))))

(event Input|KeyboardEvents|DebugKeyLeft
  (params (Key :type Key%20Structure) (ActionValue :type Input%20Action%20Value%20Structure))
  (:Pressed
    (Variables|Default|SetPressingLeft true)
    (if (not (Variables|Default|GetPressingRight))
      (bind _asbp_player_actor (Utilities|Casting|CastToBP_PlayerActor (Variables|Default|GetActiveCharacter)))
      (bind _action_wheel (Variables|/Game/RPG/Battle/PlayerPartyMembers/BP_PlayerActor.BP_PlayerActor_C|GetAction%20Wheel _asbp_player_actor)
        (:then
          (Default|RotateWheel _action_wheel -1))
        (:else
          (if (Variables|Default|GetPlayersTurn)
            (bind _currentability (Variables|Default|GetCurrentAbility)
              (:then
                (bind _output (Default|SelectUp _currentability (Variables|/Game/RPG/BP_BattleCharacterController.BP_BattleCharacterController_C|GetActiveParty (Variables|Default|GetPlayerController)) (Variables|Default|GetEnemyParty) (Variables|Default|GetTargetedActor)))
                (CallFunction|SetNewSelectedTarget _output))
              (:else))
            (else
              (Development|PrintString "Hello")))))))
  (:Released
    (Variables|Default|SetPressingLeft false)))

(event Input|KeyboardEvents|DebugKeyRight
  (params (Key :type Key%20Structure) (ActionValue :type Input%20Action%20Value%20Structure))
  (:Pressed
    (Variables|Default|SetPressingRight true)
    (if (not (Variables|Default|GetPressingLeft))
      (bind _asbp_player_actor (Utilities|Casting|CastToBP_PlayerActor (Variables|Default|GetActiveCharacter)))
      (bind _action_wheel (Variables|/Game/RPG/Battle/PlayerPartyMembers/BP_PlayerActor.BP_PlayerActor_C|GetAction%20Wheel _asbp_player_actor)
        (:then
          (Default|RotateWheel _action_wheel 1))
        (:else
          (if (Variables|Default|GetPlayersTurn)
            (bind _currentability (Variables|Default|GetCurrentAbility)
              (:then
                (bind _output (Default|SelectDown _currentability (Variables|/Game/RPG/BP_BattleCharacterController.BP_BattleCharacterController_C|GetActiveParty (Variables|Default|GetPlayerController)) (Variables|Default|GetEnemyParty) (Variables|Default|GetTargetedActor)))
                (CallFunction|SetNewSelectedTarget _output))
              (:else)))))))
  (:Released
    (Variables|Default|SetPressingRight false)))

(event Input|KeyboardEvents|DebugKeyEnter
  (params (Key :type Key%20Structure) (ActionValue :type Input%20Action%20Value%20Structure))
  (:Pressed
    (if (Variables|Default|GetPlayersTurn)
      (bind _currentability (Variables|Default|GetCurrentAbility)
        (:then
          (Default|ActivateAbility _currentability))
        (:else
          (bind _asbp_player_actor (Utilities|Casting|CastToBP_PlayerActor (Variables|Default|GetActiveCharacter)))
          (Default|SelectActionSlot (Variables|/Game/RPG/Battle/PlayerPartyMembers/BP_PlayerActor.BP_PlayerActor_C|GetAction%20Wheel _asbp_player_actor)))))))

(event Input|KeyboardEvents|DebugKeyBackspace
  (params (Key :type Key%20Structure) (ActionValue :type Input%20Action%20Value%20Structure))
  (:Pressed
    (bind _currentability (Variables|Default|GetCurrentAbility)
      (:then
        (Actor|DestroyActor _currentability)
        (Default|ClearAbilities (Variables|Default|GetBattleHUD))
        (bind _asbp_player_actor (Utilities|Casting|CastToBP_PlayerActor (Variables|Default|GetActiveCharacter)))
        (Default|SpawnWheel _asbp_player_actor))
      (:else
        (Development|PrintString "Hello")
        (Default|ClearAbilities (Variables|Default|GetBattleHUD))
        (CallFunction|SetPlayerMenu)
        (Class|BPITurnBasedCombat|SetTargeted(Message) (Variables|Default|GetTargetedActor) false)
        (bind _asbp_player_actor_2 (Utilities|Casting|CastToBP_PlayerActor (Variables|Default|GetActiveCharacter)))
        (Variables|/Game/RPG/Battle/BP_ActionWheel.BP_ActionWheel_C|SetbSlotSelected (Variables|/Game/RPG/Battle/PlayerPartyMembers/BP_PlayerActor.BP_PlayerActor_C|GetAction%20Wheel _asbp_player_actor_2) false)))))

(event Input|KeyboardEvents|DebugKeyA
  (params (Key :type Key%20Structure) (ActionValue :type Input%20Action%20Value%20Structure))
  (:Pressed
    (Variables|Default|SetPressingLeft true)
    (if (not (Variables|Default|GetPressingRight))
      (bind _asbp_player_actor (Utilities|Casting|CastToBP_PlayerActor (Variables|Default|GetActiveCharacter)))
      (bind _action_wheel (Variables|/Game/RPG/Battle/PlayerPartyMembers/BP_PlayerActor.BP_PlayerActor_C|GetAction%20Wheel _asbp_player_actor)
        (:then
          (Default|RotateWheel _action_wheel -1))
        (:else
          (if (Variables|Default|GetPlayersTurn)
            (bind _currentability (Variables|Default|GetCurrentAbility)
              (:then
                (bind _output (Default|SelectUp _currentability (Variables|/Game/RPG/BP_BattleCharacterController.BP_BattleCharacterController_C|GetActiveParty (Variables|Default|GetPlayerController)) (Variables|Default|GetEnemyParty) (Variables|Default|GetTargetedActor)))
                (CallFunction|SetNewSelectedTarget _output))
              (:else))
            (else
              (Development|PrintString "Hello")))))))
  (:Released
    (Variables|Default|SetPressingLeft false)))

(event Input|KeyboardEvents|DebugKeyD
  (params (Key :type Key%20Structure) (ActionValue :type Input%20Action%20Value%20Structure))
  (:Pressed
    (Variables|Default|SetPressingRight true)
    (if (not (Variables|Default|GetPressingLeft))
      (bind _asbp_player_actor (Utilities|Casting|CastToBP_PlayerActor (Variables|Default|GetActiveCharacter)))
      (bind _action_wheel (Variables|/Game/RPG/Battle/PlayerPartyMembers/BP_PlayerActor.BP_PlayerActor_C|GetAction%20Wheel _asbp_player_actor)
        (:then
          (Default|RotateWheel _action_wheel 1))
        (:else
          (if (Variables|Default|GetPlayersTurn)
            (bind _currentability (Variables|Default|GetCurrentAbility)
              (:then
                (bind _output (Default|SelectDown _currentability (Variables|/Game/RPG/BP_BattleCharacterController.BP_BattleCharacterController_C|GetActiveParty (Variables|Default|GetPlayerController)) (Variables|Default|GetEnemyParty) (Variables|Default|GetTargetedActor)))
                (CallFunction|SetNewSelectedTarget _output))
              (:else)))))))
  (:Released
    (Variables|Default|SetPressingRight false)))

(event Input|KeyboardEvents|DebugKeyW
  (params (Key :type Key%20Structure) (ActionValue :type Input%20Action%20Value%20Structure))
  (:Pressed
    (if (Variables|Default|GetPlayersTurn)
      (Variables|Default|GetCurrentAbility
        (:then
          (bind _output (Default|SelectOtherParty (Variables|Default|GetCurrentAbility) (Variables|/Game/RPG/BP_BattleCharacterController.BP_BattleCharacterController_C|GetActiveParty (Variables|Default|GetPlayerController)) (Variables|Default|GetEnemyParty) (Variables|Default|GetTargetedActor)))
          (CallFunction|SetNewSelectedTarget _output))
        (:else)))))

(event Input|KeyboardEvents|DebugKeyS
  (params (Key :type Key%20Structure) (ActionValue :type Input%20Action%20Value%20Structure))
  (:Pressed
    (if (Variables|Default|GetPlayersTurn)
      (Variables|Default|GetCurrentAbility
        (:then
          (bind _output (Default|SelectOtherParty (Variables|Default|GetCurrentAbility) (Variables|/Game/RPG/BP_BattleCharacterController.BP_BattleCharacterController_C|GetActiveParty (Variables|Default|GetPlayerController)) (Variables|Default|GetEnemyParty) (Variables|Default|GetTargetedActor)))
          (CallFunction|SetNewSelectedTarget _output))
        (:else)))))

(fn ConstructionScript)

(fn GetBattleCharacters
  (LocalVariables|SetOutputArray (Variables|/Game/RPG/BP_BattleCharacterController.BP_BattleCharacterController_C|GetActiveParty (Variables|Default|GetPlayerController)))
  (for _array_element (Variables|Default|GetEnemyParty)
    (Utilities|Array|AddUnique (LocalVariables|GetOutputArray) _array_element))
  (return (LocalVariables|GetOutputArray)))

(fn SetTurnOrder
  (if (Variables|Default|GetPlayer%20Advantage)
    (Variables|Default|SetTurnOrderActors (CallFunction|GetBattleCharacters) :!label _label)
    (elif (Variables|Default|GetEnemy%20Advantage)
      (for _array_element (Variables|Default|GetEnemyParty)
        (Utilities|Array|AddUnique (Variables|Default|GetTurnOrderActors) _array_element))
      (for _array_element_2 (Variables|/Game/RPG/BP_BattleCharacterController.BP_BattleCharacterController_C|GetActiveParty (Variables|Default|GetPlayerController))
        (Utilities|Array|AddUnique (Variables|Default|GetTurnOrderActors) _array_element_2))
      (else
        (goto _label)))))

(fn SetSelectionbyIndex
  (params (Index :type Integer))
  (bind _groundparty (LocalVariables|GetGroundParty))
  (bind _currentability (Variables|Default|GetCurrentAbility)
    (:then
      (switch Utilities|FlowControl|Switch|SwitchonE_TargetSelection (Variables|/Game/RPG/Battle/Abilities/BP_TurnBasedAbility.BP_TurnBasedAbility_C|GetSelection _currentability)
        (:NewEnumerator0
          (CallFunction|SelectioninArray Index (Variables|Default|GetEnemyParty)))
        (:NewEnumerator2
          (CallFunction|SelectioninArray Index (Variables|/Game/RPG/BP_BattleCharacterController.BP_BattleCharacterController_C|GetActiveParty (Variables|Default|GetPlayerController))))
        (:NewEnumerator4
          (for _array_element (Variables|Default|GetEnemyParty)
            (bind _asbp_enemy_actor (Utilities|Casting|CastToBP_EnemyActor _array_element))
            (if (Variables|/Game/RPG/Battle/BP_TurnBasedActor.BP_TurnBasedActor_C|GetbGrounded _asbp_enemy_actor)
              (Utilities|Array|AddUnique _groundparty _array_element)))
          (CallFunction|SelectioninArray Index _groundparty))))
    (:else)))

(fn SelectioninArray
  (params (Index :type Integer) (Array :type Array%20of%20Actor%20Object%20References))
  (bind _returnvalue (Utilities|Array|LastIndex Array))
  (if (> Index _returnvalue)
    (Variables|Default|SetSelectionIndex 0)
    (elif (< Index 0)
      (Variables|Default|SetSelectionIndex _returnvalue)
      (else
        (Variables|Default|SetSelectionIndex Index))))
  (Variables|Default|SetTargetedActor (Utilities|Array|Get(acopy) Array (Variables|Default|GetSelectionIndex))))

(fn SetNewSelectedTarget
  (params (Actor :type Actor%20Object%20Reference))
  (Utilities|IsValid Actor
    (:Is%20Valid
      (Class|BPITurnBasedCombat|SetTargeted(Message) (Variables|Default|GetTargetedActor) false)
      (bind _output_get (Variables|Default|SetTargetedActor Actor))
      (Class|BPITurnBasedCombat|SetTargeted(Message) _output_get true)
      (bind _targetedactor (Variables|Default|GetTargetedActor)
        (:then
          (CallFunction|SetNewPartyMemberTarget _targetedactor (Utilities|Array|FindItem (Variables|/Game/RPG/BP_BattleCharacterController.BP_BattleCharacterController_C|GetActiveParty (Variables|Default|GetPlayerController)) (Variables|Default|GetActiveCharacter)))
          (Default|SetTargetInfo (Variables|Default|GetBattleHUD) (Variables|Default|GetTargetedActor)))
        (:else
          (Development|PrintString "INVALID TARGET" true true "(R=1.000000,G=0.060992,B=0.000000,A=1.000000)"))))))

(fn SetNewPartyMemberTarget
  (params (TargetActor :type Actor%20Object%20Reference) (PartyMemberIndex :type Integer))
  (bind _component (Class|BPITurnBasedCombat|GetTurnBasedComponent(Message) (Utilities|Array|Get(acopy) (Variables|/Game/RPG/BP_BattleCharacterController.BP_BattleCharacterController_C|GetActiveParty (Variables|Default|GetPlayerController)) PartyMemberIndex)))
  (Variables|/Game/RPG/AC_AbilitySystem.AC_AbilitySystem_C|SetTargetActor _component TargetActor))

(fn LoseBattle
  (Development|PrintString "YOU LOSE" true true "(R=1.000000,G=0.005937,B=0.839136,A=1.000000)" 1e+01)
  (for _array_element (Variables|/Game/RPG/BP_BattleCharacterController.BP_BattleCharacterController_C|GetActiveParty (Variables|Default|GetPlayerController))
    (bind _component (Class|BPITurnBasedCombat|GetTurnBasedComponent(Message) _array_element))
    (bind _currentvalue_withmods_ (Default|GetAttributeCurrent _component "HP"))
    (if (> _currentvalue_withmods_ 0.0)
      (Development|PrintString "alive")
      (return)))
  (Variables|Default|SetStopBattle true)
  (Game|OpenLevel(byObjectReference) "/Game/RPG/Levels/MainMenu.MainMenu"))

(fn AddXPtoAward
  (params (XP :type Integer))
  (for _array_element (Variables|/Game/RPG/BP_BattleCharacterController.BP_BattleCharacterController_C|GetActiveParty (Variables|Default|GetPlayerController))
    (bind _component (Class|BPITurnBasedCombat|GetTurnBasedComponent(Message) _array_element))
    (bind _currentvalue_withmods_ (Default|GetAttributeCurrent _component "HP"))
    (if (> _currentvalue_withmods_ 0.0)
      (LocalVariables|SetPreviousValue (.Value (Utilities|Map|Find (Variables|Default|GetXPToReward) _array_element)))
      (else
        (LocalVariables|SetPreviousValue 0)))
    (Utilities|Map|Add (Variables|Default|GetXPToReward) _array_element (+ (LocalVariables|GetPreviousValue) XP))))

(fn AwardXP
  (bind _xptoreward (Variables|Default|GetXPToReward))
  (bind _playercontroller (Variables|Default|GetPlayerController))
  (bind _keys (Utilities|Map|Keys _xptoreward))
  (for _array_element _keys
    (bind _asbp_player_actor (Utilities|Casting|CastToBP_PlayerActor _array_element))
    (if (.ReturnValue (Utilities|Map|Find _xptoreward _array_element))
      (bind _component (Default|GetTurnBasedComponent _asbp_player_actor))
      (bind _currentvalue_withmods_ (Default|GetAttributeCurrent _component "HP"))
      (if (> _currentvalue_withmods_ 0.0)
        (Default|GiveXp _asbp_player_actor (.Value (Utilities|Map|Find _xptoreward _array_element)))
        (Variables|/Game/RPG/BP_BattleCharacterController.BP_BattleCharacterController_C|SetPlayerFirstStrike _playercontroller false)
        (Variables|/Game/RPG/BP_BattleCharacterController.BP_BattleCharacterController_C|SetEnemyFirstStrike _playercontroller false)))))