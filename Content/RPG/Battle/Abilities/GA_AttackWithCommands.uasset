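; GA_AttackWithCommands is a turn-based battle attack ability that deals fixed damage to the owning ability component's target actor.
; On activation it commits, waits through a short delay, prints a debug string and spawns the NS_Damage Niagara effect at the target's location.
; It gets the target's turn-based component via a message call, applies a negative HP effect to it and ends the ability.
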(event EventBeginPlay)

(event Collision|EventActorBeginOverlap
  (params (OtherActor :type Actor%20Object%20Reference)))

(event EventTick
  (params (DeltaSeconds :type Float%20%28single-precision%29)))

(event EventActivateAbility
  (bind _owningabilitycomponent (Variables|Default|GetOwningAbilityComponent))
  (bind _targetactor (Variables|/Game/RPG/AC_AbilitySystem.AC_AbilitySystem_C|GetTargetActor _owningabilitycomponent))
  (bind _commited (CallFunction|CommitAbility))
  (if _commited
    (Utilities|FlowControl|Delay 2.0)
    (Development|PrintString "Attack Ability")
    (bind _component (Class|BPITurnBasedCombat|GetTurnBasedComponent(Message) _targetactor))
    (Niagara|SpawnSystematLocation "/Game/RPG/Niagara/NS_Damage.NS_Damage" (Transformation|GetActorLocation _targetactor))
    (Default|ApplyEffecttoTarget _owningabilitycomponent "NewEnumerator0" _component "HP" "NewEnumerator4" "NewEnumerator0" -1e+01)
    (CallFunction|EndAbility)))

(fn ConstructionScript
  (|CallParentFunction))