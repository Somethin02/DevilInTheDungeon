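; Turn-based battle ability actor that handles cost commitment, target selection and attack power calculation.
; CommitAbility applies the cost through the owning ability component, or destroys the actor if the ability is disallowed; EndAbility also destroys it.
; Target navigation cycles within or across parties using a wrapping search filtered by CanSelect, which accepts everything here.
; Attack power combines ATK minus target DEF, ability power and an elemental weakness modifier from a data table.
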(event Custom|ActivateAbility
  (bind _hud (Variables|Default|GetHUD)
    (:then
      (Default|ClearTargets _hud))
    (:else)))

(event Custom|EndAbility
  (Default|CallAbilityEnd self)
  (Actor|DestroyActor))

(event Custom|SelectAbility)

(fn ConstructionScript)

(fn CommitAbility
  (bind _cost (Variables|Default|GetCost))
  (bind _can_do (Default|CanDoAbility1 (Variables|Default|GetOwningAbilityComponent) (Utilities|GetClass self)))
  (if _can_do
    (bind _hud (Variables|Default|GetHUD)
      (:then
        (Default|ClearTargets _hud))
      (:else
        _))
    (Default|ApplyEffecttoSelf (Variables|Default|GetOwningAbilityComponent) "NewEnumerator0" (.name _cost) "NewEnumerator4" "NewEnumerator0" (* (.cost _cost) -1.0))
    (return true)
    (else
      (Actor|DestroyActor)
      (return false))))

(fn SelectUp
  (params (PlayerParty :type Array%20of%20Actor%20Object%20References) (EnemyParty :type Array%20of%20Actor%20Object%20References) (CurrentlySelected :type Actor%20Object%20Reference))
  (if (Utilities|Array|ContainsItem PlayerParty CurrentlySelected)
    (bind _output (CallFunction|LoopOverArraywithWrap PlayerParty true (- (Utilities|Array|FindItem PlayerParty CurrentlySelected) 1)))
    (return _output)
    (else
      (bind _output_2 (CallFunction|LoopOverArraywithWrap EnemyParty true (- (Utilities|Array|FindItem EnemyParty CurrentlySelected) 1)))
      (return _output_2))))

(fn SelectDown
  (params (PlayerParty :type Array%20of%20Actor%20Object%20References) (EnemyParty :type Array%20of%20Actor%20Object%20References) (CurrentlySelected :type Actor%20Object%20Reference))
  (if (Utilities|Array|ContainsItem PlayerParty CurrentlySelected)
    (bind _output (CallFunction|LoopOverArraywithWrap PlayerParty false (+ (Utilities|Array|FindItem PlayerParty CurrentlySelected) 1)))
    (return _output)
    (else
      (bind _output_2 (CallFunction|LoopOverArraywithWrap EnemyParty false (+ (Utilities|Array|FindItem EnemyParty CurrentlySelected) 1)))
      (return _output_2))))

(fn SelectOtherParty
  (params (PlayerParty :type Array%20of%20Actor%20Object%20References) (EnemyParty :type Array%20of%20Actor%20Object%20References) (CurrentlySelected :type Actor%20Object%20Reference))
  (if (Utilities|Array|ContainsItem PlayerParty CurrentlySelected)
    (bind _output (CallFunction|LoopOverArraywithWrap EnemyParty false (Utilities|Array|FindItem PlayerParty CurrentlySelected)))
    (return _output)
    (else
      (bind _output_2 (CallFunction|LoopOverArraywithWrap PlayerParty false (Utilities|Array|FindItem EnemyParty CurrentlySelected)))
      (return _output_2))))

(fn LoopOverArraywithWrap
  (params (Array :type Array%20of%20Actor%20Object%20References) (CountDown :type Boolean) (StartIndex :type Integer))
  (bind _returnvalue (Utilities|Array|Length Array))
  (bind _output_get (LocalVariables|SetStartingIndex (+ StartIndex _returnvalue)))
  (LocalVariables|SetGoalIndex (+ _output_get (* (Math|Integer|SelectInt -1 1 CountDown) _returnvalue)))
  (bind _output_get_2 (LocalVariables|SetCurrentIndex (LocalVariables|GetStartingIndex)))
  (bind _canselect (CallFunction|CanSelect (Utilities|Array|Get(acopy) Array (Math|Integer|%(Integer) _output_get_2 _returnvalue)) :!label _label))
  (if _canselect
    (return (Utilities|Array|Get(acopy) Array (Math|Integer|%(Integer) _output_get_2 _returnvalue)))
    (else
      (if CountDown
        (Math|Integer|DecrementInt (LocalVariables|GetCurrentIndex)
          (:%20%20
            _))
        (else
          (Math|Integer|IncrementInt (LocalVariables|GetCurrentIndex)
            (:%20%20
              _))))
      (if (select CountDown (< (LocalVariables|GetCurrentIndex) (LocalVariables|GetGoalIndex)) (> (LocalVariables|GetCurrentIndex) (LocalVariables|GetGoalIndex)))
        (return 0)
        (else
          (goto _label))))))

(fn CanSelect
  (params (Actor :type Actor%20Object%20Reference))
  (return true))

(fn UpdateSelectedTarget
  (params (PlayerParty :type Array%20of%20Actor%20Object%20References) (EnemyParty :type Array%20of%20Actor%20Object%20References) (CurrentlySelected :type Actor%20Object%20Reference))
  (bind _returnvalue (Utilities|Array|FindItem PlayerParty CurrentlySelected))
  (bind _returnvalue_2 (Utilities|Array|FindItem EnemyParty CurrentlySelected))
  (bind _canselect (CallFunction|CanSelect CurrentlySelected))
  (if _canselect
    (return CurrentlySelected)
    (elif (Utilities|Array|ContainsItem PlayerParty CurrentlySelected)
      (bind _output (CallFunction|LoopOverArraywithWrap PlayerParty false _returnvalue))
      (Utilities|IsValid _output
        (:Is%20Valid
          (return _output))
        (:Is%20Not%20Valid
          (bind _output_2 (CallFunction|LoopOverArraywithWrap EnemyParty false _returnvalue))
          (return _output_2)))
      (else
        (bind _output_3 (CallFunction|LoopOverArraywithWrap EnemyParty false _returnvalue_2))
        (Utilities|IsValid _output_3
          (:Is%20Valid
            (return _output_3))
          (:Is%20Not%20Valid
            (bind _output_4 (CallFunction|LoopOverArraywithWrap PlayerParty false _returnvalue_2))
            (return _output_4)))))))

(fn CheckElementalAffinity
  (params (TargetActor :type Actor%20Object%20Reference))
  (bind _asbp_turn_based_actor (Utilities|Casting|CastToBP_TurnBasedActor TargetActor))
  (bind _returnvalue (Utilities|GetDataTableRow "/Game/RPG/Data/DataTables/DT_ElementalAffinities.DT_ElementalAffinities" (Utilities|Name|EnumtoName (Variables|/Game/RPG/Battle/BP_TurnBasedActor.BP_TurnBasedActor_C|GetElement _asbp_turn_based_actor)))
    (:then
      (if (not (== (Utilities|Array|FindItem (.Weakness (Utilities|Struct|BreakS_ElementalAffinities _returnvalue)) (Variables|Default|GetElement)) -1))
        (Variables|Default|SetElementModifier 1)))))

(fn CalcAttackPower
  (bind _owningabilitycomponent (Variables|Default|GetOwningAbilityComponent))
  (bind _currentvalue_withmods_ (Default|GetAttributeCurrent _owningabilitycomponent "ATK"))
  (Development|PrintString (Utilities|String|ToString(Float) _currentvalue_withmods_) true true "(R=1.000000,G=0.896004,B=0.019579,A=1.000000)" 5.0)
  (bind _asbp_turn_based_actor (Utilities|Casting|CastToBP_TurnBasedActor (Variables|/Game/RPG/AC_AbilitySystem.AC_AbilitySystem_C|GetTargetActor _owningabilitycomponent)))
  (bind _currentvalue_withmods__2 (Default|GetAttributeCurrent (Variables|/Game/RPG/Battle/BP_TurnBasedActor.BP_TurnBasedActor_C|GetAC_AbilitySystem _asbp_turn_based_actor) "DEF"))
  (return (Math|Float|Floor (+ (+ (- _currentvalue_withmods_ _currentvalue_withmods__2) (Variables|Default|GetAbilityAttackPower)) (Variables|Default|GetElementModifier)))))