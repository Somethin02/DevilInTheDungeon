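; BP_BirdsEye is an overworld trigger that briefly shows a bird's-eye camera shot, judging by its name.
; When BP_OverworldPlayerCharacter enters its Sphere, it disables that character's input and blends the view to its Cam.
; After a short hold, it blends back to the character and restores input using timed delays.
; Nothing disables the trigger afterward, so re-entering can replay the shot.
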(event OnComponentBeginOverlap(Sphere)
  (params (OverlappedComponent :type Primitive%20Component%20Object%20Reference) (OtherActor :type Actor%20Object%20Reference) (OtherComp :type Primitive%20Component%20Object%20Reference) (OtherBodyIndex :type Integer) (bFromSweep :type Boolean) (SweepResult :type Hit%20Result%20Structure%20%28by%20ref%29))
  (bind _asbp_overworld_player_character (Utilities|Casting|CastToBP_OverworldPlayerCharacter OtherActor))
  (Input|DisableInput OtherActor (Game|GetPlayerController 0))
  (Game|Player|SetViewTargetwithBlend (Game|GetPlayerController 0) (Variables|Default|GetCam) 3.0 "VTBlend_Linear" 0.0 false)
  (Utilities|FlowControl|Delay 3.0)
  (Utilities|FlowControl|Delay 0.2)
  (Game|Player|SetViewTargetwithBlend (Game|GetPlayerController 0) _asbp_overworld_player_character 3.0 "VTBlend_Linear" 0.0 false)
  (Utilities|FlowControl|Delay 3.0)
  (Input|EnableInput OtherActor (Game|GetPlayerController 0)))

(event EventBeginPlay)

(event Collision|EventActorBeginOverlap
  (params (OtherActor :type Actor%20Object%20Reference)))

(event EventTick
  (params (DeltaSeconds :type Float%20%28single-precision%29)))

(fn ConstructionScript)