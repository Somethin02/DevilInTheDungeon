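; Manager that populates an RPG overworld floor with enemies when the level finishes building, via the LevelFinished event.
; It derives a random stream from the game instance's master seed plus a salt, then spawns a random enemy class at each BP_OverworldEnemySpawner.
; Each enemy receives an encounter layout from the seed-shuffled floor encounter table, keeping the last row whose first enemy matches its battle counterpart.
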(event EventLevelFinished
  (bind _asgi_rpg (Utilities|Casting|CastToGI_RPG (Game|GetGameInstance)))
  (Variables|Default|SetEnemySpawnSeed (Math|Random|MakeRandomStream (+ (Class|KismetMathLibrary|BreakRandomStream (Variables|/Game/GI_RPG.GI_RPG_C|GetMasterSeed _asgi_rpg)) (Variables|Default|GetEnemySpawnSalt))))
  (bind _outactors (Actor|GetAllActorsOfClass "/Game/RPG/BP_OverworldEnemySpawner.BP_OverworldEnemySpawner_C"))
  (for _array_element _outactors
    (bind _output_get (Variables|Default|SetEnemySpawn (.OutItem (Utilities|Array|RandomFromStream (Variables|Default|GetEnemySelection) (Variables|Default|GetEnemySpawnSeed)))))
    (bind _returnvalue (Game|SpawnActorfromClass _output_get (Transformation|GetWorldTransform (Variables|/Game/RPG/BP_OverworldEnemySpawner.BP_OverworldEnemySpawner_C|GetDefaultSceneRoot _array_element)) "AlwaysSpawn" "MultiplyWithRoot" 0 0))
    (Variables|Default|SetSpawnedEnemy _returnvalue)
    (bind _outrownames (DataTable|GetDataTableRowNames (Variables|Default|GetFloorEncounterTable)))
    (Utilities|Array|ShuffleFromStream _outrownames (Variables|Default|GetEnemySpawnSeed))
    (for _array_element_2 _outrownames
      (bind _returnvalue_2 (Utilities|GetDataTableRow (Variables|Default|GetFloorEncounterTable) _array_element_2)
        (:then
          (if (== (Variables|/Game/RPG/BP_OverworldEnemy.BP_OverworldEnemy_C|GetCorrespondingBattleEnemy (Variables|Default|GetSpawnedEnemy)) (.Enemy1 (Utilities|Struct|BreakS_BasicEncounter _returnvalue_2)))
            (Variables|/Game/RPG/BP_OverworldEnemy.BP_OverworldEnemy_C|SetEnemyLayout (Variables|Default|GetSpawnedEnemy) _returnvalue_2)))))))

(fn ConstructionScript)