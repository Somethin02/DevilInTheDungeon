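; RPG battle character controller that creates and holds the player's three-member party.
; On BeginPlay it spawns three hidden, collision-free BP_PlayerActors at its own transform into ActiveParty, adds the default input mapping context and caches the overworld player character.
; SpawnPlayerCharacters reruns that setup when the party is empty.
; OpenNextLevel always opens TestMap, while the Floor increment is unconnected.
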(event Custom|SpawnPlayerCharacters
  (if (Utilities|Array|IsEmpty (Variables|Default|GetActiveParty))
    (Development|PrintString "character spawn")
    (bind _returnvalue (Game|SpawnActorfromClass "/Game/RPG/Battle/PlayerPartyMembers/BP_PlayerActor.BP_PlayerActor_C" (Transformation|GetActorTransform) "Undefined" "MultiplyWithRoot" 0 0))
    (Rendering|SetActorHiddenInGame _returnvalue true)
    (Collision|SetActorEnableCollision _returnvalue false)
    (Variables|Default|SetPlayer1 _returnvalue)
    (bind _returnvalue_2 (Game|SpawnActorfromClass "/Game/RPG/Battle/PlayerPartyMembers/BP_PlayerActor.BP_PlayerActor_C" (Transformation|GetActorTransform) "Undefined" "MultiplyWithRoot" 0 0))
    (Rendering|SetActorHiddenInGame _returnvalue_2 true)
    (Collision|SetActorEnableCollision _returnvalue_2 false)
    (Variables|Default|SetPlayer2 _returnvalue_2)
    (bind _returnvalue_3 (Game|SpawnActorfromClass "/Game/RPG/Battle/PlayerPartyMembers/BP_PlayerActor.BP_PlayerActor_C" (Transformation|GetActorTransform) "Undefined" "MultiplyWithRoot" 0 0))
    (Rendering|SetActorHiddenInGame _returnvalue_3 true)
    (Collision|SetActorEnableCollision _returnvalue_3 false)
    (Variables|Default|SetPlayer3 _returnvalue_3)
    (for _array_element (Utilities|Array|MakeArray (Variables|Default|GetPlayer1) (Variables|Default|GetPlayer2) (Variables|Default|GetPlayer3))
      (Utilities|IsValid _array_element
        (:Is%20Valid
          (Rendering|SetActorHiddenInGame true))))
    (Variables|Default|SetActiveParty (Utilities|Array|MakeArray (Variables|Default|GetPlayer1) (Variables|Default|GetPlayer2) (Variables|Default|GetPlayer3)))
    (Input|AddMappingContext (PlayerController|LocalPlayerSubsystems|GetEnhancedInputLocalPlayerSubsystem (Game|GetPlayerController 0)) "/Game/Input/IMC_Default.IMC_Default" 0 "(bIgnoreAllPressedKeysUntilRelease=True,bForceImmediately=False,bNotifyUserSettings=False)")
    (bind _asbp_overworld_player_character (Utilities|Casting|CastToBP_OverworldPlayerCharacter (Game|GetPlayerCharacter 0)))
    (Variables|Default|SetAs%20BP%20Overworld%20Player%20Character _asbp_overworld_player_character)))

(event Custom|OpenNextLevel
  (Game|OpenLevel(byObjectReference) "/Game/RPG/Levels/TestMap.TestMap"))

(event EventBeginPlay
  (bind _returnvalue (Game|SpawnActorfromClass "/Game/RPG/Battle/PlayerPartyMembers/BP_PlayerActor.BP_PlayerActor_C" (Transformation|GetActorTransform) "Undefined" "MultiplyWithRoot" 0 0))
  (Rendering|SetActorHiddenInGame _returnvalue true)
  (Collision|SetActorEnableCollision _returnvalue false)
  (Variables|Default|SetPlayer1 _returnvalue)
  (bind _returnvalue_2 (Game|SpawnActorfromClass "/Game/RPG/Battle/PlayerPartyMembers/BP_PlayerActor.BP_PlayerActor_C" (Transformation|GetActorTransform) "Undefined" "MultiplyWithRoot" 0 0))
  (Rendering|SetActorHiddenInGame _returnvalue_2 true)
  (Collision|SetActorEnableCollision _returnvalue_2 false)
  (Variables|Default|SetPlayer2 _returnvalue_2)
  (bind _returnvalue_3 (Game|SpawnActorfromClass "/Game/RPG/Battle/PlayerPartyMembers/BP_PlayerActor.BP_PlayerActor_C" (Transformation|GetActorTransform) "Undefined" "MultiplyWithRoot" 0 0))
  (Rendering|SetActorHiddenInGame _returnvalue_3 true)
  (Collision|SetActorEnableCollision _returnvalue_3 false)
  (Variables|Default|SetPlayer3 _returnvalue_3)
  (for _array_element (Utilities|Array|MakeArray (Variables|Default|GetPlayer1) (Variables|Default|GetPlayer2) (Variables|Default|GetPlayer3))
    (Utilities|IsValid _array_element
      (:Is%20Valid
        (Rendering|SetActorHiddenInGame true))))
  (Variables|Default|SetActiveParty (Utilities|Array|MakeArray (Variables|Default|GetPlayer1) (Variables|Default|GetPlayer2) (Variables|Default|GetPlayer3)))
  (Input|AddMappingContext (PlayerController|LocalPlayerSubsystems|GetEnhancedInputLocalPlayerSubsystem (Game|GetPlayerController 0)) "/Game/Input/IMC_Default.IMC_Default" 0 "(bIgnoreAllPressedKeysUntilRelease=True,bForceImmediately=False,bNotifyUserSettings=False)")
  (bind _asbp_overworld_player_character (Utilities|Casting|CastToBP_OverworldPlayerCharacter (Game|GetPlayerCharacter 0)))
  (Variables|Default|SetAs%20BP%20Overworld%20Player%20Character _asbp_overworld_player_character))

(fn ConstructionScript)