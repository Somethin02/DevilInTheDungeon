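; Overworld enemy spawn manager that spawns a random enemy class at a supplied transform and assigns it a battle layout.
; SpawnEnemy picks from EnemySelection using a seeded stream, then shuffles the floor encounter table rows.
; The last row whose Enemy1 matches the enemy's battle counterpart becomes its layout.
; LevelFinished is empty; the master-seed-plus-salt setup and loop over placed spawners are disconnected and never run.
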(event Custom|SpawnEnemy
  (params (SpawnTransform :type Transform))
  (bind _output_get (Variables|Default|SetEnemySpawn (.OutItem (Utilities|Array|RandomFromStream (Variables|Default|GetEnemySelection) (Variables|Default|GetEnemySpawnSeed)))))
  (bind _returnvalue (Game|SpawnActorfromClass :Class _output_get :SpawnTransform SpawnTransform :CollisionHandlingOverride "AlwaysSpawn" :TransformScaleMethod "MultiplyWithRoot" :Instigator 0))
  (Variables|Default|SetSpawnedEnemy _returnvalue)
  (bind _outrownames (DataTable|GetDataTableRowNames (Variables|Default|GetFloorEncounterTable)))
  (Utilities|Array|ShuffleFromStream _outrownames (Variables|Default|GetEnemySpawnSeed))
  (for _array_element _outrownames
    (bind _returnvalue_2 (Utilities|GetDataTableRow (Variables|Default|GetFloorEncounterTable) _array_element)
      (:then
        (if (== (Variables|/Game/RPG/Overworld/BP_OverworldEnemy.BP_OverworldEnemy_C|GetCorrespondingBattleEnemy (Variables|Default|GetSpawnedEnemy)) (.Enemy1 (Utilities|Struct|BreakS_BasicEncounter _returnvalue_2)))
          (Variables|/Game/RPG/Overworld/BP_OverworldEnemy.BP_OverworldEnemy_C|SetEnemyLayout (Variables|Default|GetSpawnedEnemy) _returnvalue_2))))))

(event EventLevelFinished)

(fn ConstructionScript)