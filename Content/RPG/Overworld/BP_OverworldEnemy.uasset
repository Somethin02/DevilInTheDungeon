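; Overworld enemy character that wanders its surroundings and starts an RPG battle when its hurtbox overlaps the player.
; Roaming loops AI MoveTo calls to random nearby reachable points, retrying after a delay on success or failure.
; Contact passes both first-strike flags and the enemy layout to the battle controller, halts roaming and calls the player's EnterBattle.
; Die spawns a coin spawner, notifies the overlapping room via EnemyDeathCheck, then destroys the actor.
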(event OnComponentBeginOverlap(Hurtbox)
  (params (OverlappedComponent :type Primitive%20Component%20Object%20Reference) (OtherActor :type Actor%20Object%20Reference) (OtherComp :type Primitive%20Component%20Object%20Reference) (OtherBodyIndex :type Integer) (bFromSweep :type Boolean) (SweepResult :type Hit%20Result%20Structure%20%28by%20ref%29))
  (bind _asbp_overworld_player_character (Utilities|Casting|CastToBP_OverworldPlayerCharacter OtherActor))
  (Variables|Default|SetPlayerTransform (Transformation|GetActorTransform _asbp_overworld_player_character))
  (bind _asbp_battle_character_controller (Utilities|Casting|CastToBP_BattleCharacterController (Game|GetPlayerController 0)))
  (Variables|/Game/RPG/BP_BattleCharacterController.BP_BattleCharacterController_C|SetPlayerFirstStrike _asbp_battle_character_controller (Variables|/Game/RPG/Overworld/BP_OverworldPlayerCharacter.BP_OverworldPlayerCharacter_C|GetFirstStrike _asbp_overworld_player_character))
  (Variables|/Game/RPG/BP_BattleCharacterController.BP_BattleCharacterController_C|SetEnemyFirstStrike _asbp_battle_character_controller (Variables|Default|GetFirstStrike))
  (Variables|/Game/RPG/BP_BattleCharacterController.BP_BattleCharacterController_C|SetEnemyLayout _asbp_battle_character_controller (Variables|Default|GetEnemyLayout))
  (Components|Movement|StopMovementImmediately (Variables|Character|GetCharacterMovement))
  (Variables|Default|SetbRoam false)
  (Default|EnterBattle _asbp_overworld_player_character self))

(event Custom|SpawnDrops
  (bind _mesh (Variables|Character|GetMesh))
  (Collision|SetCollisionEnabled _mesh "NoCollision")
  (Development|SetHiddeninGame _mesh false false)
  (CallFunction|SpawnCoins 5))

(event Custom|SpawnCoins
  (params (CoinCount :type Integer))
  (bind _returnvalue (Game|SpawnActorfromClass "/Game/RPG/BP_CoinSpawner.BP_CoinSpawner_C" (Transformation|GetWorldTransform (Variables|Default|GetDropSpawnpoint)) "Undefined" "MultiplyWithRoot" 0 5 0))
  (Default|SpawnCoins _returnvalue))

(event Custom|Roaming
  (if (Variables|Default|GetbRoam)
    (AI|AIMoveTo self (.RandomLocation (AI|Navigation|GetRandomReachablePointinRadius (Transformation|GetActorLocation) 5e+02 0 0)) 0 5.0 false
      (:then
        (Development|PrintString "roaming"))
      (:OnSuccess
        (Utilities|FlowControl|Delay 1.0 :!label _label)
        (CallFunction|Roaming))
      (:OnFail
        (Development|PrintString "Failure to roam")
        (goto _label)))))

(event Custom|Die
  (CallFunction|SpawnDrops)
  (bind _asbp_parent_room (Utilities|Casting|CastToBP_ParentRoom (Utilities|Array|Get(acopy) (Collision|GetOverlappingActors (Variables|Collision|GetCapsuleComponent) "/Game/RPG/DungeonGeneration/BP_ParentRoom.BP_ParentRoom_C" :!class /Script/Engine.PrimitiveComponent))))
  (Default|EnemyDeathCheck _asbp_parent_room)
  (Actor|DestroyActor))

(event EventBeginPlay
  (Variables|Default|SetAIControllerClass "/Script/AIModule.AIController")
  (CallFunction|Roaming))

(fn ConstructionScript)